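; Pressure plate that switches on a referenced BP_NewInteractDoor when the player steps on it.
; Player overlap lowers the plate by timeline; leaving raises it unless the door's required time is completed.
; Timeline updates feed a retriggerable delay using the door's required time, which is not cancelled on exit.
; For multi-input doors, the plate decrements the input count once, opening at zero; unwired timer tests remain.
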(event OnComponentBeginOverlap(Trigger)
  (params (OverlappedComponent :type Primitive%20Component%20Object%20Reference) (OtherActor :type Actor%20Object%20Reference) (OtherComp :type Primitive%20Component%20Object%20Reference) (OtherBodyIndex :type Integer) (bFromSweep :type Boolean) (SweepResult :type Hit%20Result%20Structure%20%28by%20ref%29))
  (bind _door_ref (Variables|Default|GetDoor%20Ref))
  (bind _door_ref_2 (Variables|Default|GetDoor%20Ref))
  (bind _door_ref_3 (Variables|Default|GetDoor%20Ref))
  (bind _asbp_new_interact_door (Utilities|Casting|CastToBP_NewInteractDoor _door_ref))
  (bind _asbp_new_interact_door_2 (Utilities|Casting|CastToBP_NewInteractDoor _door_ref_2))
  (bind _asbp_new_interact_door_3 (Utilities|Casting|CastToBP_NewInteractDoor _door_ref_3))
  (Utilities|Casting|CastToBP_Player OtherActor)
  (Variables|Default|SetIs%20Active%20? true)
  (bind _height (Timeline|Timeline Play)
    (:Update
      (Transformation|SetRelativeLocation (Variables|Default|GetPlate) (Math|Vector|MakeVector 0.0 0.0 (Math|Float|Lerp 1e+01 -2.0 _height)) false false)
      (if (Variables|Default|GetIs%20Active%20?)
        (Utilities|FlowControl|RetriggerableDelay (Variables|/Game/Elements/Interactibles(Loris)/BP_NewInteractDoor.BP_NewInteractDoor_C|GetTime%20Required%20On%20Plate _asbp_new_interact_door_3))
        (Variables|/Game/Elements/Interactibles(Loris)/BP_NewInteractDoor.BP_NewInteractDoor_C|SetRequired%20Time%20Completed%20? _asbp_new_interact_door_3 true)
        (if (Variables|/Game/Elements/Interactibles(Loris)/BP_NewInteractDoor.BP_NewInteractDoor_C|GetRequired%20Time%20Completed%20? _asbp_new_interact_door)
          (if (Variables|/Game/Elements/Interactibles(Loris)/BP_NewInteractDoor.BP_NewInteractDoor_C|GetNeeds%20Multiple%20Inputs%20? _asbp_new_interact_door)
            (if (<= (Variables|/Game/Elements/Interactibles(Loris)/BP_NewInteractDoor.BP_NewInteractDoor_C|GetInputs%20Amount _asbp_new_interact_door) 0) :!label _label
              _
              (else
                (Utilities|FlowControl|DoOnce false
                  (:Completed
                    (bind _output_get (Variables|/Game/Elements/Interactibles(Loris)/BP_NewInteractDoor.BP_NewInteractDoor_C|SetInputs%20Amount _asbp_new_interact_door_2 (- (Variables|/Game/Elements/Interactibles(Loris)/BP_NewInteractDoor.BP_NewInteractDoor_C|GetInputs%20Amount _asbp_new_interact_door_2) 1)))
                    (Development|PrintString (Utilities|String|ToString(Integer) _output_get))
                    (goto _label))))))
          (Default|SwitchON _asbp_new_interact_door))))))

(event OnComponentEndOverlap(Trigger)
  (params (OverlappedComponent :type Primitive%20Component%20Object%20Reference) (OtherActor :type Actor%20Object%20Reference) (OtherComp :type Primitive%20Component%20Object%20Reference) (OtherBodyIndex :type Integer))
  (bind _door_ref (Variables|Default|GetDoor%20Ref))
  (bind _door_ref_2 (Variables|Default|GetDoor%20Ref))
  (bind _door_ref_3 (Variables|Default|GetDoor%20Ref))
  (bind _asbp_new_interact_door (Utilities|Casting|CastToBP_NewInteractDoor _door_ref))
  (bind _asbp_new_interact_door_2 (Utilities|Casting|CastToBP_NewInteractDoor _door_ref_2))
  (bind _asbp_new_interact_door_3 (Utilities|Casting|CastToBP_NewInteractDoor _door_ref_3))
  (Utilities|Casting|CastToBP_Player OtherActor)
  (if (not (Variables|/Game/Elements/Interactibles(Loris)/BP_NewInteractDoor.BP_NewInteractDoor_C|GetRequired%20Time%20Completed%20? (.AsBP%20New%20Interact%20Door (Utilities|Casting|CastToBP_NewInteractDoor (Variables|Default|GetDoor%20Ref)))))
    (Variables|Default|SetIs%20Active%20? false)
    (bind _height (Timeline|Timeline Reverse)
      (:Update
        (Transformation|SetRelativeLocation (Variables|Default|GetPlate) (Math|Vector|MakeVector 0.0 0.0 (Math|Float|Lerp 1e+01 -2.0 _height)) false false)
        (if (Variables|Default|GetIs%20Active%20?)
          (Utilities|FlowControl|RetriggerableDelay (Variables|/Game/Elements/Interactibles(Loris)/BP_NewInteractDoor.BP_NewInteractDoor_C|GetTime%20Required%20On%20Plate _asbp_new_interact_door_3))
          (Variables|/Game/Elements/Interactibles(Loris)/BP_NewInteractDoor.BP_NewInteractDoor_C|SetRequired%20Time%20Completed%20? _asbp_new_interact_door_3 true)
          (if (Variables|/Game/Elements/Interactibles(Loris)/BP_NewInteractDoor.BP_NewInteractDoor_C|GetRequired%20Time%20Completed%20? _asbp_new_interact_door)
            (if (Variables|/Game/Elements/Interactibles(Loris)/BP_NewInteractDoor.BP_NewInteractDoor_C|GetNeeds%20Multiple%20Inputs%20? _asbp_new_interact_door)
              (if (<= (Variables|/Game/Elements/Interactibles(Loris)/BP_NewInteractDoor.BP_NewInteractDoor_C|GetInputs%20Amount _asbp_new_interact_door) 0) :!label _label
                _
                (else
                  (Utilities|FlowControl|DoOnce false
                    (:Completed
                      (bind _output_get (Variables|/Game/Elements/Interactibles(Loris)/BP_NewInteractDoor.BP_NewInteractDoor_C|SetInputs%20Amount _asbp_new_interact_door_2 (- (Variables|/Game/Elements/Interactibles(Loris)/BP_NewInteractDoor.BP_NewInteractDoor_C|GetInputs%20Amount _asbp_new_interact_door_2) 1)))
                      (Development|PrintString (Utilities|String|ToString(Integer) _output_get))
                      (goto _label))))))
            (Default|SwitchON _asbp_new_interact_door)))))))

(event Custom|TimerHeld
  ;[0 1 1] Test
)

(event Custom|TimerDone
  ;[0 1 1] Test
)

(event EventTick
  (params (DeltaSeconds :type Float%20%28single-precision%29))
  ;[0 1 1] Test
)

(fn ConstructionScript)