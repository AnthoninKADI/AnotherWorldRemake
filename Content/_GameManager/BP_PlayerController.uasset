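; Player controller that turns Enhanced Input into BP_Player actions: movement, look, sprint, crouch, shooting, camera aim, pause and a sidekick follow toggle.
; BeginPlay adds the mapping context, sets max acceleration and clamps camera pitch.
; Moving and shooting snap pawn yaw to the camera, and shooting passes input hold time to the weapon.
; Sprint and crouch swap walk speeds, while aim toggles timeline-driven spring arm zoom.
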(event Input|EnhancedActionEvents|EnhancedInputActionIA_Follow
  (params (ActionValue :type Boolean) (ElapsedSeconds :type Float%20%28double-precision%29) (TriggeredSeconds :type Float%20%28double-precision%29) (InputAction :type Input%20Action%20Object%20Reference :default "/Game/_GameManager/Input/Actions/IA_Follow.IA_Follow"))
  ;[0 0.2211 1] Switch Sidekick follow enable / disable
  (:Canceled
    (if (Variables|Default|GetAllow%20Follow?) :!label _label
      (Variables|Default|SetAllow%20Follow? false)
      (else
        (Variables|Default|SetAllow%20Follow? true))))
  (:Completed
    (goto _label)))

(event Input|EnhancedActionEvents|EnhancedInputActionIA_Pause
  (params (ActionValue :type Boolean) (ElapsedSeconds :type Float%20%28double-precision%29) (TriggeredSeconds :type Float%20%28double-precision%29) (InputAction :type Input%20Action%20Object%20Reference :default "/Game/_GameManager/Input/Actions/UI_Inputs/IA_Pause.IA_Pause"))
  (bind _returnvalue (Game|GetPlayerController 0))
  (:Triggered
    (bind _returnvalue_2 (UserInterface|CreateWidget "/Game/UI/W_PauseMenu.W_PauseMenu_C" _returnvalue))
    (UserInterface|Viewport|AddtoViewport _returnvalue_2 0)
    (Game|SetGamePaused true)
    (Input|SetInputModeUIOnly _returnvalue (Variables|/Game/UI/W_PauseMenu.W_PauseMenu_C|GetResume _returnvalue_2) "DoNotLock" false)))

(event Input|EnhancedActionEvents|EnhancedInputActionIA_Shoot
  (params (ActionValue :type Boolean) (ElapsedSeconds :type Float%20%28double-precision%29) (TriggeredSeconds :type Float%20%28double-precision%29) (InputAction :type Input%20Action%20Object%20Reference :default "/Game/_GameManager/Input/Actions/IA_Shoot.IA_Shoot"))
  (bind _returnvalue (Pawn|GetControlledPawn))
  (bind _weapon (Variables|Default|GetWeapon))
  (bind _returnvalue_2 (Transformation|GetActorRotation _returnvalue))
  (bind (_roll _pitch) (Math|Rotator|BreakRotator _returnvalue_2))
  (:Canceled
    ;[0.35 0.45 1] Rotate Player Forward To Camera Forward
    (Transformation|SetActorRelativeRotation _returnvalue (Math|Rotator|MakeRotator _roll _pitch (.yaw (Variables|/Script/Engine.SceneComponent|GetRelativeRotation (Variables|/Script/Engine.PlayerCameraManager|GetTransformComponent (Game|GetPlayerCameraManager 0))))) true :!label _label)
    (if (Utilities|IsValid _weapon)
      (Default|Shoot _weapon ElapsedSeconds)))
  (:Completed
    (goto _label)))

(event Input|EnhancedActionEvents|EnhancedInputActionIA_Look
  (params (ActionValue :type Vector%202D%20Structure) (ElapsedSeconds :type Float%20%28double-precision%29) (TriggeredSeconds :type Float%20%28double-precision%29) (InputAction :type Input%20Action%20Object%20Reference :default "/Game/_GameManager/Input/Actions/IA_Look.IA_Look"))
  (bind (_x _y) (Math|Vector2D|BreakVector2D ActionValue))
  (:Triggered
    (Class|PlayerController|AddYawInput _x)
    (Class|PlayerController|AddPitchInput _y)))

(event Input|EnhancedActionEvents|EnhancedInputActionIA_Crouch
  (params (ActionValue :type Boolean) (ElapsedSeconds :type Float%20%28double-precision%29) (TriggeredSeconds :type Float%20%28double-precision%29) (InputAction :type Input%20Action%20Object%20Reference :default "/Game/_GameManager/Input/Actions/IA_Crouch.IA_Crouch"))
  (bind _returnvalue (Pawn|GetControlledPawn))
  (bind _returnvalue_2 (Game|GetPlayerCharacter 0))
  (:Canceled
    (Utilities|FlowControl|Delay 0.15 :!label _label)
    ;[1 1 1] Toggle Crouching
    (bind _isa (Utilities|FlowControl|FlipFlop)
      (:A
        (Variables|Default|SetIs%20Crouching%20? _isa)
        (Character|Crouch _returnvalue_2)
        (bind _asbp_player (Utilities|Casting|CastToBP_Player _returnvalue))
        (Variables|/Script/Engine.CharacterMovementComponent|SetMaxWalkSpeed (Variables|/Script/Engine.Character|GetCharacterMovement _asbp_player) (Variables|/Script/AnotherWorldRemake.Player_Main|GetMaxCrouchSpeed _asbp_player)))
      (:B
        (Variables|Default|SetIs%20Crouching%20? _isa)
        (Character|UnCrouch _returnvalue_2)
        (bind _asbp_player_2 (Utilities|Casting|CastToBP_Player _returnvalue))
        (Variables|/Script/Engine.CharacterMovementComponent|SetMaxWalkSpeed (Variables|/Script/Engine.Character|GetCharacterMovement _asbp_player_2) (Variables|/Script/AnotherWorldRemake.Player_Main|GetMaxWalkSpeed _asbp_player_2)))))
  (:Completed
    (goto _label)))

(event Input|EnhancedActionEvents|EnhancedInputActionIA_Sprint
  (params (ActionValue :type Boolean) (ElapsedSeconds :type Float%20%28double-precision%29) (TriggeredSeconds :type Float%20%28double-precision%29) (InputAction :type Input%20Action%20Object%20Reference :default "/Game/_GameManager/Input/Actions/IA_Sprint.IA_Sprint"))
  (bind _returnvalue (Pawn|GetControlledPawn))
  (:Triggered
    (bind _asbp_player (Utilities|Casting|CastToBP_Player _returnvalue))
    (Variables|/Script/Engine.CharacterMovementComponent|SetMaxWalkSpeed (Variables|/Script/Engine.Character|GetCharacterMovement _asbp_player) (Variables|/Script/AnotherWorldRemake.Player_Main|GetMaxRunSpeed _asbp_player)))
  (:Canceled
    (bind _asbp_player_2 (Utilities|Casting|CastToBP_Player _returnvalue :!label _label))
    (Variables|/Script/Engine.CharacterMovementComponent|SetMaxWalkSpeed (Variables|/Script/Engine.Character|GetCharacterMovement _asbp_player_2) (Variables|/Script/AnotherWorldRemake.Player_Main|GetMaxWalkSpeed _asbp_player_2)))
  (:Completed
    (goto _label)))

(event Input|EnhancedActionEvents|EnhancedInputActionIA_Move
  (params (ActionValue :type Vector%202D%20Structure) (ElapsedSeconds :type Float%20%28double-precision%29) (TriggeredSeconds :type Float%20%28double-precision%29) (InputAction :type Input%20Action%20Object%20Reference :default "/Game/_GameManager/Input/Actions/IA_Move.IA_Move"))
  (bind (_x _y) (Math|Vector2D|BreakVector2D ActionValue))
  (bind _returnvalue (Pawn|GetControlRotation :!class /Script/Engine.Controller))
  (bind _returnvalue_2 (Pawn|GetControlledPawn))
  (bind _returnvalue_3 (Transformation|GetActorRotation _returnvalue_2))
  (bind (_roll _pitch) (Math|Rotator|BreakRotator _returnvalue_3))
  (:Triggered
    (Pawn|Input|AddMovementInput (Pawn|GetControlledPawn) (Math|Vector|GetForwardVector (Math|Rotator|MakeRotator 0.0 0.0 (.yaw (Pawn|GetControlRotation :!class /Script/Engine.Controller)))) _y false)
    (Pawn|Input|AddMovementInput (Pawn|GetControlledPawn) (Math|Vector|GetRightVector (Math|Rotator|MakeRotator (.roll _returnvalue) 0.0 (.yaw _returnvalue))) _x false)
    ;[0.35 0.45 1] Rotate Player Forward To Camera Forward
    (Transformation|SetActorRelativeRotation _returnvalue_2 (Math|Rotator|MakeRotator _roll _pitch (.yaw (Variables|/Script/Engine.SceneComponent|GetRelativeRotation (Variables|/Script/Engine.PlayerCameraManager|GetTransformComponent (Game|GetPlayerCameraManager 0))))) true)))

(event Input|EnhancedActionEvents|EnhancedInputActionIA_CamAim
  (params (ActionValue :type Boolean) (ElapsedSeconds :type Float%20%28double-precision%29) (TriggeredSeconds :type Float%20%28double-precision%29) (InputAction :type Input%20Action%20Object%20Reference :default "/Game/_GameManager/Input/Actions/IA_CamAim.IA_CamAim"))
  (bind _returnvalue (Game|GetPlayerCharacter 0))
  (bind _zoomed_arm_length (Variables|Default|GetZoomed%20Arm%20Length))
  (bind _base_arm_length (Variables|Default|GetBase%20Arm%20Length))
  (bind _asbp_player (Utilities|Casting|CastToBP_Player _returnvalue))
  (bind _springarm (Variables|/Game/Characters/Player/BP_Player.BP_Player_C|GetSpringArm _asbp_player))
  (:Canceled
    ;[1 1 1] Toggle
    (Utilities|FlowControl|FlipFlop :!label _label
      (:A
        ;[0.3663 0.2918 0.1274] Smoothing
        (bind _cam_lerp (Timeline|Timeline PlayFromStart)
          (:Update
            (Variables|/Script/Engine.SpringArmComponent|SetTargetArmLength _springarm (Math|Float|Lerp _base_arm_length _zoomed_arm_length _cam_lerp))
            ;[1 1 1] Set to the lenght of the Timelines
            (Utilities|FlowControl|Delay 0.5))))
      (:B
        (bind _cam_lerp_2 (Timeline|Timeline%202 PlayFromStart)
          (:Update
            (Variables|/Script/Engine.SpringArmComponent|SetTargetArmLength _springarm (Math|Float|Lerp _zoomed_arm_length _base_arm_length _cam_lerp_2))
            (Utilities|FlowControl|Delay 0.5))))))
  (:Completed
    (goto _label)))

(event EventBeginPlay
  (bind _returnvalue (Game|GetPlayerCameraManager 0))
  (Input|AddMappingContext (PlayerController|LocalPlayerSubsystems|GetEnhancedInputLocalPlayerSubsystem) "/Game/_GameManager/Input/IMC_Default.IMC_Default" 0 "(bIgnoreAllPressedKeysUntilRelease=True,bForceImmediately=False)")
  ;[1 1 1] Acceleration Set
  (bind _asbp_player (Utilities|Casting|CastToBP_Player (Pawn|GetControlledPawn)))
  (Variables|/Script/Engine.CharacterMovementComponent|SetMaxAcceleration (Variables|/Script/Engine.Character|GetCharacterMovement _asbp_player) (Variables|/Script/AnotherWorldRemake.Player_Main|GetAcceleration2 _asbp_player))
  ;[0 1 0] Camera Clamp
  (Variables|/Script/Engine.PlayerCameraManager|SetViewPitchMax _returnvalue (Variables|Default|GetView%20Pitch%20Max))
  (Variables|/Script/Engine.PlayerCameraManager|SetViewPitchMin _returnvalue (Variables|Default|GetView%20Pitch%20Min)))

(fn ConstructionScript)