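; BP_TriggerActor is a pressure plate or button that players and followers activate to switch a linked Target.
; It counts overlaps, then changes the emissive material, plays a sound and moves the plate via a timeline.
; While active, a retriggerable delay enforces the Target's required time before switching it on.
; Multi-input Targets wait until all registered triggers are active; ShouldStay governs switch-off on release, latching once all are active.
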(event OnComponentBeginOverlap(Trigger)
  (params (OverlappedComponent :type Primitive%20Component%20Object%20Reference) (OtherActor :type Actor%20Object%20Reference) (OtherComp :type Primitive%20Component%20Object%20Reference) (OtherBodyIndex :type Integer) (bFromSweep :type Boolean) (SweepResult :type Hit%20Result%20Structure%20%28by%20ref%29))
  (bind _plate_to_move (Variables|ref|GetPlate%20To%20Move))
  (bind _activatorcount (Variables|Default|GetActivatorCount))
  (bind _target (Variables|Ref|GetTarget))
  (bind _base_y_pos (Variables|BasePos|GetBase%20Y%20pos))
  (bind _base_z_pos (Variables|BasePos|GetBase%20Z%20pos))
  (bind _target_2 (Variables|Ref|GetTarget))
  (bind _triggered_on_sound (Variables|Sound|GetTriggered%20On%20Sound))
  (bind _triggered_off_sound (Variables|Sound|GetTriggered%20Off%20Sound))
  (bind _target_3 (Variables|Ref|GetTarget))
  (bind _target_4 (Variables|Ref|GetTarget))
  (bind _target_5 (Variables|Ref|GetTarget))
  (bind _triggers (Variables|/Game/Elements/BP_ActivatableActor.BP_ActivatableActor_C|GetTriggers _target_3))
  (bind _allactive (Variables|/Game/Elements/BP_ActivatableActor.BP_ActivatableActor_C|GetAllActive _target_4))
  (bind _returnvalue (Utilities|Array|Length _allactive))
  (bind _returnvalue_2 (Utilities|Set|Length _triggers))
  (bind _returnvalue_3 (== _returnvalue _returnvalue_2))
  (Utilities|Casting|CastToBP_Player OtherActor
    (:then
      _)
    (:CastFailed
      (Utilities|Casting|CastToBP_FollowerBase OtherActor)))
  ;[1 1 1] keeps track of all people currently activating trigger, sends positive nessage when nobody is
  (Math|Integer|IncrementInt _activatorcount
    (:%20%20
      (if (> _activatorcount 0)
        (Variables|Default|SetIsActive? true)
        (Rendering|Material|SetMaterial (Variables|ref|GetEmisive) 1 (Variables|Mat|GetGreen))
        (Utilities|IsValid _triggered_on_sound
          (:Is%20Valid
            (Audio|PlaySoundatLocation _triggered_on_sound (Transformation|GetWorldLocation (Variables|Default|GetDefaultSceneRoot)) "0, 0, 0" 1.0 1.0 0.0 0 0 0 0)
            (bind _height (Timeline|Timeline Play)
              (:Update
                (if (Variables|Default|GetIsButton?)
                  (Transformation|SetRelativeLocation _plate_to_move (Math|Vector|MakeVector (Math|Float|Lerp _base_z_pos (- _base_z_pos 5.0) _height) _base_y_pos (Variables|BasePos|GetBase%20Z%20pos)) false false)
                  (else
                    (Transformation|SetRelativeLocation _plate_to_move (Math|Vector|MakeVector (Variables|BasePos|GetBase%20X%20pos) _base_y_pos (Math|Float|Lerp _base_z_pos (- _base_z_pos 5.0) _height)) false false)))
                (if (Variables|Default|GetIsActive?)
                  (Utilities|IsValid _target_5
                    (:Is%20Valid
                      (Utilities|FlowControl|RetriggerableDelay (Variables|/Game/Elements/BP_ActivatableActor.BP_ActivatableActor_C|GetTime%20Required%20On%20Plate _target_5))
                      (Variables|/Game/Elements/BP_ActivatableActor.BP_ActivatableActor_C|SetRequired%20Time%20Completed%20? _target_5 true)
                      (if (Variables|/Game/Elements/BP_ActivatableActor.BP_ActivatableActor_C|GetRequired%20Time%20Completed%20? _target_2)
                        (if (Variables|/Game/Elements/BP_ActivatableActor.BP_ActivatableActor_C|GetNeeds%20Multiple%20Inputs%20? _target_2)
                          (Utilities|Array|AddUnique (Variables|/Game/Elements/BP_ActivatableActor.BP_ActivatableActor_C|GetAllActive (Variables|Ref|GetTarget)) (Utilities|String|StringToName (Utilities|GetObjectName self)))
                          (if _returnvalue_3
                            (Default|SwitchON _target :!label _label)
                            (else
                              (Default|SwitchOFF _target :!label _label_2)))
                          (else
                            (goto _label))))))
                  (elif (Variables|Default|GetShouldStay?)
                    (if (not _returnvalue_3)
                      (Utilities|Array|RemoveItem (Variables|/Game/Elements/BP_ActivatableActor.BP_ActivatableActor_C|GetAllActive (Variables|Ref|GetTarget)) (Utilities|String|StringToName (Utilities|GetObjectName self)))
                      (goto _label_2)))))))
          (:Is%20Not%20Valid
            (Timeline|Timeline Play)))
        (else
          (Variables|Default|SetIsActive? false)
          (Rendering|Material|SetMaterial (Variables|ref|GetEmisive) 1 (Variables|Mat|GetRed))
          (Utilities|IsValid _triggered_off_sound
            (:Is%20Valid
              (Audio|PlaySoundatLocation _triggered_off_sound (Transformation|GetWorldLocation (Variables|Default|GetDefaultSceneRoot)) "0, 0, 0" 1.0 1.0 0.0 0 0 0 0)
              (Timeline|Timeline Reverse))
            (:Is%20Not%20Valid
              (Timeline|Timeline Reverse))))))))

(event OnComponentEndOverlap(Trigger)
  (params (OverlappedComponent :type Primitive%20Component%20Object%20Reference) (OtherActor :type Actor%20Object%20Reference) (OtherComp :type Primitive%20Component%20Object%20Reference) (OtherBodyIndex :type Integer))
  (bind _plate_to_move (Variables|ref|GetPlate%20To%20Move))
  (bind _activatorcount (Variables|Default|GetActivatorCount))
  (bind _target (Variables|Ref|GetTarget))
  (bind _base_y_pos (Variables|BasePos|GetBase%20Y%20pos))
  (bind _base_z_pos (Variables|BasePos|GetBase%20Z%20pos))
  (bind _target_2 (Variables|Ref|GetTarget))
  (bind _triggered_on_sound (Variables|Sound|GetTriggered%20On%20Sound))
  (bind _triggered_off_sound (Variables|Sound|GetTriggered%20Off%20Sound))
  (bind _target_3 (Variables|Ref|GetTarget))
  (bind _target_4 (Variables|Ref|GetTarget))
  (bind _target_5 (Variables|Ref|GetTarget))
  (bind _target_6 (Variables|Ref|GetTarget))
  (bind _triggers (Variables|/Game/Elements/BP_ActivatableActor.BP_ActivatableActor_C|GetTriggers _target_4))
  (bind _allactive (Variables|/Game/Elements/BP_ActivatableActor.BP_ActivatableActor_C|GetAllActive _target_5))
  (bind _returnvalue (Utilities|Array|Length _allactive))
  (bind _returnvalue_2 (Utilities|Set|Length _triggers))
  (bind _returnvalue_3 (== _returnvalue _returnvalue_2))
  (Utilities|IsValid _target_3
    (:Is%20Valid
      (if (Variables|/Game/Elements/BP_ActivatableActor.BP_ActivatableActor_C|GetRequired%20Time%20Completed%20? _target_3)
        (if (Variables|Default|GetShouldStay?)
          _
          (else
            _)))
      ;[1 1 1] keeps track of all people currently activating trigger, sends positive nessage when nobody is
      (Math|Integer|DecrementInt _activatorcount
        (:%20%20
          (if (> _activatorcount 0)
            (Variables|Default|SetIsActive? true)
            (Rendering|Material|SetMaterial (Variables|ref|GetEmisive) 1 (Variables|Mat|GetGreen))
            (Utilities|IsValid _triggered_on_sound
              (:Is%20Valid
                (Audio|PlaySoundatLocation _triggered_on_sound (Transformation|GetWorldLocation (Variables|Default|GetDefaultSceneRoot)) "0, 0, 0" 1.0 1.0 0.0 0 0 0 0)
                (bind _height (Timeline|Timeline Play)
                  (:Update
                    (if (Variables|Default|GetIsButton?)
                      (Transformation|SetRelativeLocation _plate_to_move (Math|Vector|MakeVector (Math|Float|Lerp _base_z_pos (- _base_z_pos 5.0) _height) _base_y_pos (Variables|BasePos|GetBase%20Z%20pos)) false false)
                      (else
                        (Transformation|SetRelativeLocation _plate_to_move (Math|Vector|MakeVector (Variables|BasePos|GetBase%20X%20pos) _base_y_pos (Math|Float|Lerp _base_z_pos (- _base_z_pos 5.0) _height)) false false)))
                    (if (Variables|Default|GetIsActive?)
                      (Utilities|IsValid _target_6
                        (:Is%20Valid
                          (Utilities|FlowControl|RetriggerableDelay (Variables|/Game/Elements/BP_ActivatableActor.BP_ActivatableActor_C|GetTime%20Required%20On%20Plate _target_6))
                          (Variables|/Game/Elements/BP_ActivatableActor.BP_ActivatableActor_C|SetRequired%20Time%20Completed%20? _target_6 true)
                          (if (Variables|/Game/Elements/BP_ActivatableActor.BP_ActivatableActor_C|GetRequired%20Time%20Completed%20? _target_2)
                            (if (Variables|/Game/Elements/BP_ActivatableActor.BP_ActivatableActor_C|GetNeeds%20Multiple%20Inputs%20? _target_2)
                              (Utilities|Array|AddUnique (Variables|/Game/Elements/BP_ActivatableActor.BP_ActivatableActor_C|GetAllActive (Variables|Ref|GetTarget)) (Utilities|String|StringToName (Utilities|GetObjectName self)))
                              (if _returnvalue_3
                                (Default|SwitchON _target :!label _label)
                                (else
                                  (Default|SwitchOFF _target :!label _label_2)))
                              (else
                                (goto _label))))))
                      (elif (Variables|Default|GetShouldStay?)
                        (if (not _returnvalue_3)
                          (Utilities|Array|RemoveItem (Variables|/Game/Elements/BP_ActivatableActor.BP_ActivatableActor_C|GetAllActive (Variables|Ref|GetTarget)) (Utilities|String|StringToName (Utilities|GetObjectName self)))
                          (goto _label_2)))))))
              (:Is%20Not%20Valid
                (Timeline|Timeline Play)))
            (else
              (Variables|Default|SetIsActive? false)
              (Rendering|Material|SetMaterial (Variables|ref|GetEmisive) 1 (Variables|Mat|GetRed))
              (Utilities|IsValid _triggered_off_sound
                (:Is%20Valid
                  (Audio|PlaySoundatLocation _triggered_off_sound (Transformation|GetWorldLocation (Variables|Default|GetDefaultSceneRoot)) "0, 0, 0" 1.0 1.0 0.0 0 0 0 0)
                  (Timeline|Timeline Reverse))
                (:Is%20Not%20Valid
                  (Timeline|Timeline Reverse))))))))))

(event EventBeginPlay
  (Utilities|FlowControl|Delay 0.2)
  (bind _target (Variables|Ref|GetTarget)
    (:then
      (Default|Notify _target self false)
      (if (Variables|Default|GetIsTarget?)
        (Variables|ref|SetPlate%20To%20Move 0)
        (Variables|ref|SetEmisive 0)
        (else
          (Variables|BasePos|SetBase%20X%20pos (.x (Variables|/Script/Engine.SceneComponent|GetRelativeLocation (Variables|ref|GetPlate%20To%20Move))))
          (Variables|BasePos|SetBase%20Y%20pos (.y (Variables|/Script/Engine.SceneComponent|GetRelativeLocation (Variables|ref|GetPlate%20To%20Move))))
          (Variables|BasePos|SetBase%20Z%20pos (.z (Variables|/Script/Engine.SceneComponent|GetRelativeLocation (Variables|ref|GetPlate%20To%20Move)))))))
    (:else)))

(fn ConstructionScript)