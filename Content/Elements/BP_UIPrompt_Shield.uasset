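; BP_UIPrompt_Shield is a trigger-volume actor that shows a UI prompt, apparently for the shield going by its name.
; When the player character enters the Box, it adds its Widget to the viewport only if BP_PlayerController's SidekickActivated is set, and removes it on exit.
; A DoOnce check on entry leads to nothing, and the Widget is not created in these graphs.
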(event OnComponentBeginOverlap(Box)
  (params (OverlappedComponent :type Primitive%20Component%20Object%20Reference) (OtherActor :type Actor%20Object%20Reference) (OtherComp :type Primitive%20Component%20Object%20Reference) (OtherBodyIndex :type Integer) (bFromSweep :type Boolean) (SweepResult :type Hit%20Result%20Structure%20%28by%20ref%29))
  (if (== OtherActor (Game|GetPlayerCharacter 0))
    (if (Variables|/Game/_GameManager/BP_PlayerController.BP_PlayerController_C|GetSidekickActivated (.AsBP%20Player%20Controller (Utilities|Casting|CastToBP_PlayerController (Game|GetPlayerController 0))))
      (if (Variables|Default|GetDo%20Once%20?)
        (Utilities|FlowControl|DoOnce false
          (:Completed
            _)))
      (UserInterface|Viewport|AddtoViewport (Variables|Default|GetWidget) 0))))

(event OnComponentEndOverlap(Box)
  (params (OverlappedComponent :type Primitive%20Component%20Object%20Reference) (OtherActor :type Actor%20Object%20Reference) (OtherComp :type Primitive%20Component%20Object%20Reference) (OtherBodyIndex :type Integer))
  (if (== OtherActor (Game|GetPlayerCharacter 0))
    (Widget|RemovefromParent (Variables|Default|GetWidget))))

(event EventBeginPlay
  (|CallParentFunction) ; This node is disabled and will not be called.\nDrag off pins to build functionality.
)

(event Collision|EventActorBeginOverlap
  (params (OtherActor :type Actor%20Object%20Reference)))

(event EventTick
  (params (DeltaSeconds :type Float%20%28single-precision%29)))

(fn ConstructionScript
  (|CallParentFunction))