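; Activatable bridge interactible that starts retracted, with its deck and side fences hidden and non-colliding while front and back fences block the ends.
; BeginPlay adjusts end fence positions and scales to the bridge and main mesh scales, sets the Bridge Fade material collection parameter, and hands component references to parent variables before calling parent BeginPlay.
; When the player leaves the Overlap volume, it restores that closed state; no opening logic appears here.
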(event OnComponentEndOverlap(Overlap)
  (params (OverlappedComponent :type Primitive%20Component%20Object%20Reference) (OtherActor :type Actor%20Object%20Reference) (OtherComp :type Primitive%20Component%20Object%20Reference) (OtherBodyIndex :type Integer))
  (Utilities|Casting|CastToBP_Player OtherActor)
  (Utilities|FlowControl|Sequence
    (:then_0
      (Rendering|SetVisibility (Variables|Default|GetBridge%20Mesh) false false)
      (Collision|SetCollisionEnabled (Variables|Default|GetBridge%20Mesh) "NoCollision"))
    (:then_1
      (Rendering|SetVisibility (Variables|Default|GetFront%20Fence) true false)
      (Collision|SetCollisionEnabled (Variables|Default|GetFront%20Fence) "QueryAndPhysics"))
    (:then_2
      (Rendering|SetVisibility (Variables|Default|GetBack%20Fence) true false)
      (Collision|SetCollisionEnabled (Variables|Default|GetBack%20Fence) "QueryAndPhysics"))
    (:then_3
      (Rendering|SetVisibility (Variables|Default|GetR%20Side%20Fence) false false)
      (Collision|SetCollisionEnabled (Variables|Default|GetR%20Side%20Fence) "NoCollision"))
    (:then_4
      (Rendering|SetVisibility (Variables|Default|GetL%20Side%20Fence) false false)
      (Collision|SetCollisionEnabled (Variables|Default|GetL%20Side%20Fence) "NoCollision"))))

(event EventBeginPlay
  (bind _front_fence (Variables|Default|GetFront%20Fence))
  (bind _front_fence_2 (Variables|Default|GetFront%20Fence))
  (bind _back_fence (Variables|Default|GetBack%20Fence))
  (bind _back_fence_2 (Variables|Default|GetBack%20Fence))
  (bind _relativelocation (Variables|/Script/Engine.SceneComponent|GetRelativeLocation _back_fence))
  (bind _relativelocation_2 (Variables|/Script/Engine.SceneComponent|GetRelativeLocation _front_fence))
  (Utilities|FlowControl|Sequence
    (:then_0
      (Transformation|SetRelativeLocation _back_fence (Math|Vector|MakeVector (* (.x _relativelocation) (.x (Variables|/Script/Engine.SceneComponent|GetRelativeScale3D (Variables|Default|GetBridge%20Mesh)))) (.y _relativelocation) (.z _relativelocation)) false true)
      (Transformation|SetRelativeScale3D _back_fence_2 (/ (Variables|/Script/Engine.SceneComponent|GetRelativeScale3D _back_fence_2) (Variables|/Script/Engine.SceneComponent|GetRelativeScale3D (Variables|Default|GetMainMesh)))))
    (:then_1
      (Transformation|SetRelativeLocation _front_fence (Math|Vector|MakeVector (* (.x _relativelocation_2) (.x (Variables|/Script/Engine.SceneComponent|GetRelativeScale3D (Variables|Default|GetBridge%20Mesh)))) (.y _relativelocation_2) (.z _relativelocation_2)) false true)
      (Transformation|SetRelativeScale3D _front_fence_2 (/ (Variables|/Script/Engine.SceneComponent|GetRelativeScale3D _front_fence_2) (Variables|/Script/Engine.SceneComponent|GetRelativeScale3D (Variables|Default|GetMainMesh))))))
  (Utilities|FlowControl|Delay 0.2)
  (Variables|Default|SetBase%20Relative%20Scale%20X (.x (Variables|/Script/Engine.SceneComponent|GetRelativeScale3D (Variables|Default|GetBridge%20Mesh))))
  (Rendering|Material|SetScalarParameterValue "/Game/Elements/Interactibles(Loris)/MP_FadeParam.MP_FadeParam" "Bridge Fade" 1.0 :!class /Script/Engine.KismetMaterialLibrary)
  (Variables|Default|SetIsBridge? true)
  (Variables|Default|SetCube%201%20To%20Move (Variables|Default|GetBridge%20Mesh))
  (Variables|Default|SetBridge%20Actor%20Ref self)
  (Variables|Default|SetFront%20Fence%20Ref (Variables|Default|GetFront%20Fence))
  (Variables|Default|SetBack%20Fence%20Ref (Variables|Default|GetBack%20Fence))
  (Variables|Default|SetL%20Fence%20Ref (Variables|Default|GetL%20Side%20Fence))
  (Variables|Default|SetR%20Fence%20Ref (Variables|Default|GetR%20Side%20Fence))
  (Utilities|FlowControl|Sequence
    (:then_0
      (Rendering|SetVisibility (Variables|Default|GetBridge%20Mesh) false false)
      (Collision|SetCollisionEnabled (Variables|Default|GetBridge%20Mesh) "NoCollision"))
    (:then_1
      (Rendering|SetVisibility (Variables|Default|GetFront%20Fence) true false)
      (Collision|SetCollisionEnabled (Variables|Default|GetFront%20Fence) "QueryAndPhysics"))
    (:then_2
      (Rendering|SetVisibility (Variables|Default|GetBack%20Fence) true false)
      (Collision|SetCollisionEnabled (Variables|Default|GetBack%20Fence) "QueryAndPhysics"))
    (:then_3
      (Rendering|SetVisibility (Variables|Default|GetR%20Side%20Fence) false false)
      (Collision|SetCollisionEnabled (Variables|Default|GetR%20Side%20Fence) "NoCollision"))
    (:then_4
      (Rendering|SetVisibility (Variables|Default|GetL%20Side%20Fence) false false)
      (Collision|SetCollisionEnabled (Variables|Default|GetL%20Side%20Fence) "NoCollision")))
  (|CallParentFunction))

(fn ConstructionScript
  (|CallParentFunction))