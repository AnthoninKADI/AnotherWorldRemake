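; BP_Shield is a timed shield piece, parented to a BP_FullShield actor, that absorbs small bullets and lasers.
; It is one-sided: it compares its box yaw with the projectile owner's yaw and only takes hits outside an 85-degree tolerance either way.
; Hits spawn a Niagara effect, destroy the projectile and drain the parent's shared health.
; At zero, the full shield leaves its weapon's array and is destroyed with a sound.
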(event EventHitProjectile
  (params (Damage :type Integer) (Projectile :type Actor%20Object%20Reference))
  (bind _returnvalue (Transformation|GetActorLocation Projectile))
  (bind (_asbp_small_bullet _bsuccess) (Utilities|Casting|CastToBP_SmallBullet Projectile))
  (bind _asbp_laser (Utilities|Casting|CastToBP_Laser Projectile))
  (bind _destructsound (Variables|Default|GetDestructSound))
  (bind _fullshield (Variables|Default|GetFullShield))
  (bind _fullshield_2 (Variables|Default|GetFullShield))
  (bind _ownercharacter (Variables|/Game/Characters/Weapon/BP_SmallBullet.BP_SmallBullet_C|GetOwnerCharacter _asbp_small_bullet))
  (bind _shieldhealth (Variables|/Game/Characters/Weapon/BP_FullShield.BP_FullShield_C|GetShieldHealth _fullshield))
  (bind _ownercharacter_2 (Variables|/Game/Characters/Weapon/BP_Laser.BP_Laser_C|GetOwnerCharacter _asbp_laser))
  (bind _returnvalue_2 (select _bsuccess _ownercharacter _ownercharacter_2))
  (bind _returnvalue_3 (Transformation|GetActorRotation _returnvalue_2))
  (bind _yaw (Math|Rotator|BreakRotator _returnvalue_3))
  (if (not (Math|Float|InRange(Float) (.Yaw (Math|Rotator|BreakRotator (Transformation|GetWorldRotation (Variables|Default|GetBox)))) (- _yaw 85.0) (+ _yaw 85.0)))
    (Utilities|Casting|CastToBP_SmallBullet Projectile
      (:then
        (Niagara|SpawnSystematLocation "/Game/GA/VFX/NS/Character/NS_ShortBeam_MuzzleFlash.NS_ShortBeam_MuzzleFlash" _returnvalue))
      (:CastFailed
        (Utilities|Casting|CastToBP_Laser Projectile)
        (Niagara|SpawnSystematLocation "/Game/GA/VFX/NS/Character/NS_LongBeam_MuzzleFlash.NS_LongBeam_MuzzleFlash" _returnvalue)))
    (bind _output_get (Variables|/Script/AnotherWorldRemake.HealthComponent|SetCurrent _shieldhealth (- (Variables|/Script/AnotherWorldRemake.HealthComponent|GetCurrent _shieldhealth) Damage)))
    (if (<= _output_get 0)
      (Utilities|IsValid _destructsound
        (:Is%20Valid
          (Audio|PlaySoundatLocation _destructsound (Transformation|GetWorldLocation (Variables|Default|GetCube)) "0, 0, 0" 1.0 1.0 0.0 0 0 0 0))
        (:Is%20Not%20Valid
          _))
      (Utilities|Array|RemoveItem (Variables|/Game/Characters/Weapon/BP_Weapon.BP_Weapon_C|GetshieldArray (Variables|/Game/Characters/Weapon/BP_FullShield.BP_FullShield_C|GetOwningWeapon (Variables|Default|GetFullShield))) _fullshield_2)
      (Actor|DestroyActor _fullshield_2))
    (Actor|DestroyActor Projectile)))

(event EventBeginPlay
  (Actor|SetLifeSpan (Variables|Default|GetshieldLifeTime))
  (Variables|Default|SetFullShield (.AsBP%20Full%20Shield (Utilities|Casting|CastToBP_FullShield (Actor|GetParentActor self)))))

(fn ConstructionScript)