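; BP_UIPrompt is a trigger volume that shows a configurable UI prompt widget while the player character stands inside its Box.
; On the player's begin overlap, a DoOnce creates the PromptToDisplay widget, stores it in Prompt and adds it to the viewport.
; End overlap removes that widget; the DoOnce is never reset, so the prompt appears only on the first entry.
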(event OnComponentBeginOverlap(Box)
  (params (OverlappedComponent :type Primitive%20Component%20Object%20Reference) (OtherActor :type Actor%20Object%20Reference) (OtherComp :type Primitive%20Component%20Object%20Reference) (OtherBodyIndex :type Integer) (bFromSweep :type Boolean) (SweepResult :type Hit%20Result%20Structure%20%28by%20ref%29))
  (if (== OtherActor (Game|GetPlayerCharacter 0))
    (Utilities|FlowControl|DoOnce false
      (:Completed
        (bind _returnvalue (UserInterface|CreateWidget (Variables|Default|GetPromptToDisplay)))
        (bind _output_get (Variables|Default|SetPrompt _returnvalue))
        (UserInterface|Viewport|AddtoViewport _output_get 0)))))

(event OnComponentEndOverlap(Box)
  (params (OverlappedComponent :type Primitive%20Component%20Object%20Reference) (OtherActor :type Actor%20Object%20Reference) (OtherComp :type Primitive%20Component%20Object%20Reference) (OtherBodyIndex :type Integer))
  (if (== OtherActor (Game|GetPlayerCharacter 0))
    (Widget|RemovefromParent (Variables|Default|GetPrompt))))

(fn ConstructionScript)