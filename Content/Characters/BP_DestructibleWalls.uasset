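; BP_DestructibleWalls is a breakable wall whose health is reduced by laser projectile hits.
; Each HitProjectile event spawns an attached Niagara explosion, but only BP_Laser projectiles subtract damage, with remaining health printed.
; At zero health or below, the wall swaps to its broken mesh and disables collision.
; BeginPlay is wired into the same chain, so the explosion also spawns at start.
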(event EventBeginPlay
  (bind _wallhealth (Variables|Default|GetWallHealth))
  (bind _mesh (Variables|Default|GetMesh))
  (bind _mesh_2 (Variables|Default|GetMesh))
  (Niagara|SpawnSystemAttached "/Game/GA/VFX/NS/Enviro/NS_WallExplosion.NS_WallExplosion" _mesh_2 "" (+ (Variables|/Script/Engine.SceneComponent|GetRelativeLocation _mesh_2) "10.000000,100.000000,250.000000") "0, 0, 0" "KeepRelativeOffset" false)
  (Utilities|Casting|CastToBP_Laser (stale EventHitProjectile Projectile))
  (bind _output_get (Variables|/Script/AnotherWorldRemake.HealthComponent|SetCurrent _wallhealth (- (Variables|/Script/AnotherWorldRemake.HealthComponent|GetCurrent _wallhealth) (stale EventHitProjectile Damage))))
  (Development|PrintString (Utilities|String|ToString(Integer) _output_get))
  (if (<= _output_get 0)
    ;[1 1 1] Change to destroyed wall mesh
    (Components|StaticMesh|SetStaticMesh _mesh "/Game/GA/ENVIRO/MODULAR/MESH/Walls/BreakableWalls/SM_Wall_SM_BreakableWall_After.SM_Wall_SM_BreakableWall_After")
    (Collision|SetCollisionEnabled _mesh "NoCollision")))

(event EventHitProjectile
  (params (Damage :type Integer) (Projectile :type Actor%20Object%20Reference))
  (bind _wallhealth (Variables|Default|GetWallHealth))
  (bind _mesh (Variables|Default|GetMesh))
  (bind _mesh_2 (Variables|Default|GetMesh))
  (Niagara|SpawnSystemAttached "/Game/GA/VFX/NS/Enviro/NS_WallExplosion.NS_WallExplosion" _mesh_2 "" (+ (Variables|/Script/Engine.SceneComponent|GetRelativeLocation _mesh_2) "10.000000,100.000000,250.000000") "0, 0, 0" "KeepRelativeOffset" false)
  (Utilities|Casting|CastToBP_Laser Projectile)
  (bind _output_get (Variables|/Script/AnotherWorldRemake.HealthComponent|SetCurrent _wallhealth (- (Variables|/Script/AnotherWorldRemake.HealthComponent|GetCurrent _wallhealth) Damage)))
  (Development|PrintString (Utilities|String|ToString(Integer) _output_get))
  (if (<= _output_get 0)
    ;[1 1 1] Change to destroyed wall mesh
    (Components|StaticMesh|SetStaticMesh _mesh "/Game/GA/ENVIRO/MODULAR/MESH/Walls/BreakableWalls/SM_Wall_SM_BreakableWall_After.SM_Wall_SM_BreakableWall_After")
    (Collision|SetCollisionEnabled _mesh "NoCollision")))

(fn ConstructionScript)