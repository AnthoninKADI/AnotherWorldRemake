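; Game mode Blueprint that starts the ambient music and handles player death.
; On BeginPlay it pushes the master volume mix and binds to the player's destruction, which reopens the reset level after a delay.
; A Respawn event re-runs that binding on the current player character.
; Music events fade out the ambiance, fade in a transition track, then fade the ambiance back in when that track finishes.
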(event Custom|StopCurrentAmbiance
  (Audio|Components|Audio|FadeOut (Variables|Default|GetCurrentMusic) 2.0 0.0 "Linear" :!class /Script/Engine.AudioComponent))

(event Custom|OnDeath
  (params (DestroyedActor :type Actor%20Object%20Reference))
  ;[0 0.08243 1] Checkpoints respawn system
  (Utilities|FlowControl|Delay (Variables|Default|GetRespawnTime))
  ;;[1 1 1] Reset Level
  (Game|OpenLevel(byObjectReference) (Variables|Default|GetLevelToReset)))

(event Custom|Respawn
  ;[0 0.08243 1] Checkpoints respawn system
  (bind _asbp_player (Utilities|Casting|CastToBP_Player (Game|GetPlayerCharacter 0)))
  (Game|BindEventtoOnDestroyed _asbp_player (delegate Custom|OnDeath)))

(event Custom|LaunchAmbiance
  (bind _transitionmusic (Variables|Default|GetTransitionMusic))
  (Audio|Components|Audio|SetSound _transitionmusic "/Game/Sound/Music/Music_Transition.Music_Transition")
  (Audio|Components|Audio|FadeIn _transitionmusic 2.0 1.0 0.0 "Linear" :!class /Script/Engine.AudioComponent)
  (EventDispatchers|BindEventtoOnAudioFinished _transitionmusic (delegate Custom|RelaunchAmbiance)))

(event Custom|RelaunchAmbiance
  (Audio|Components|Audio|FadeIn (Variables|Default|GetCurrentMusic) 2.0 1.0 0.0 "Linear" :!class /Script/Engine.AudioComponent))

(event EventBeginPlay
  (Utilities|FlowControl|Sequence
    (:then_0
      (Class|GameplayStatics|SetBaseSoundMix "/Game/UI/AudioSettings/MasterVolume.MasterVolume")
      (Audio|PushSoundMixModifier "/Game/UI/AudioSettings/MasterVolume.MasterVolume")
      (bind _returnvalue (Audio|SpawnSound2D "/Game/Sound/Music/Music_Ambiance.Music_Ambiance" 1.0 1.0 0.0 0))
      (Variables|Default|SetCurrentMusic _returnvalue))
    (:then_1
      ;[0 0.08243 1] Checkpoints respawn system
      (bind _asbp_player (Utilities|Casting|CastToBP_Player (Game|GetPlayerCharacter 0)))
      (Game|BindEventtoOnDestroyed _asbp_player (delegate Custom|OnDeath)))))

(fn ConstructionScript)