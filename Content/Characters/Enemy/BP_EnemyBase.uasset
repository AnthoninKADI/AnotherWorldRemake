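; Base enemy Character that chases sighted pawns, runs a placeholder crouch-and-shoot cycle and is destroyed when projectile hits deplete its health.
; Two sensing components, SightRange and ShootingRange, derive their hearing thresholds from their sight radius on BeginPlay.
; SightRange drives AIMoveTo, with a retriggerable delay that halts the chase after sightings stop.
; ShootingRange sets a flag that disables movement on subsequent sightings, while crouching and shooting only print strings.
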(event OnSeePawn(SightRange)
  (params (Pawn :type Pawn%20Object%20Reference))
  ;[1 0.8387 0] Follow Player when in Sight Range
  (Variables|Default|SetInSightZone? true)
  (Pawn|Components|CharacterMovement|SetMovementMode (Variables|Character|GetCharacterMovement) "MOVE_Walking" 0)
  (if (and (Variables|Default|GetInSightZone?) (not (Variables|Default|GetInShootingZone?)))
    (Utilities|FlowControl|Sequence
      (:then_0
        (AI|AIMoveTo self "0, 0, 0" Pawn 5.0 false))
      (:then_1
        (Utilities|FlowControl|RetriggerableDelay 1.0)
        (AI|AIMoveTo 0 (Transformation|GetActorLocation) 0 5.0 false)))
    (else
      (Pawn|Components|CharacterMovement|DisableMovement (Variables|Character|GetCharacterMovement)))))

(event OnSeePawn(ShootingRange)
  (params (Pawn :type Pawn%20Object%20Reference))
  ;[0.6776 0 1] Stop moving, crouch, shoot the player, continue moving
  (Utilities|FlowControl|Delay 0.2)
  (Variables|Default|SetInShootingZone? true)
  (Development|PrintString "Crouch")
  (Utilities|FlowControl|Delay (Variables|Default|GetAnimCrouchTime))
  (Development|PrintString "Shooting")
  (Variables|Default|SetInShootingZone? false)
  (Development|PrintString "Stop Crouch"))

(event EventHitProjectile
  (params (Damage :type Integer) (Projectile :type Actor%20Object%20Reference))
  (bind _health (Variables|Default|GetHealth))
  (bind _output_get (Variables|/Script/AnotherWorldRemake.HealthComponent|SetCurrent _health (- (Variables|/Script/AnotherWorldRemake.HealthComponent|GetCurrent _health) Damage)))
  (if (<= _output_get 0)
    (Actor|DestroyActor)))

(event EventBeginPlay
  (bind _shootingrange (Variables|Default|GetShootingRange))
  (bind _sightrange (Variables|Default|GetSightRange))
  ;[0 0.9026 1] Auto Parameter for GD with only one Variable (Sight Zone & Shooting Zone)
  (Variables|/Script/AIModule.PawnSensingComponent|SetSightRadius _sightrange (Variables|/Script/AIModule.PawnSensingComponent|GetSightRadius _sightrange))
  (Variables|/Script/AIModule.PawnSensingComponent|SetHearingThreshold _sightrange (Variables|/Script/AIModule.PawnSensingComponent|GetSightRadius _sightrange))
  (Variables|/Script/AIModule.PawnSensingComponent|SetLOSHearingThreshold _sightrange (+ (Variables|/Script/AIModule.PawnSensingComponent|GetSightRadius _sightrange) 5e+03))
  (Variables|/Script/AIModule.PawnSensingComponent|SetSightRadius _shootingrange (Variables|/Script/AIModule.PawnSensingComponent|GetSightRadius _shootingrange))
  (Variables|/Script/AIModule.PawnSensingComponent|SetHearingThreshold _shootingrange (Variables|/Script/AIModule.PawnSensingComponent|GetSightRadius _shootingrange))
  (Variables|/Script/AIModule.PawnSensingComponent|SetLOSHearingThreshold _shootingrange (+ (Variables|/Script/AIModule.PawnSensingComponent|GetSightRadius _shootingrange) 5e+03)))

(fn ConstructionScript)