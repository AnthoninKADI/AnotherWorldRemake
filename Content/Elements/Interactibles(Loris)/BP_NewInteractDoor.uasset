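; BP_NewInteractDoor is a switch-driven double door whose two cube panels slide apart and back together.
; SwitchON and SwitchOFF set the On flag and play or reverse a Timeline, whose Height value lerps the panels' mirrored Y offsets.
; While On, panels move only if RequiredTimeCompleted is true, though the timeline runs regardless; when off, they follow it unconditionally.
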(event Custom|Switch%20OFF
  (bind _cube_1 (Variables|Default|GetCube%201))
  (bind _relativelocation (Variables|/Script/Engine.SceneComponent|GetRelativeLocation _cube_1))
  (Variables|Default|SetOn%20? false)
  (bind _height (Timeline|Timeline Reverse)
    (:Update
      (if (Variables|Default|GetOn%20?)
        (if (Variables|Default|GetRequired%20Time%20Completed%20?)
          (Utilities|FlowControl|Sequence :!label _label
            (:then_0
              (Transformation|SetRelativeLocation _cube_1 (Math|Vector|MakeVector (.x _relativelocation) (Math|Float|Lerp 5e+01 1.5e+02 _height) (.z _relativelocation)) false false))
            (:then_1
              (Transformation|SetRelativeLocation (Variables|Default|GetCube%202) (Math|Vector|MakeVector (.x _relativelocation) (* (Math|Float|Lerp 5e+01 1.5e+02 _height) -1.0) (.z _relativelocation)) false false))))
        (else
          (goto _label))))))

(event Custom|Switch%20ON
  (bind _cube_1 (Variables|Default|GetCube%201))
  (bind _relativelocation (Variables|/Script/Engine.SceneComponent|GetRelativeLocation _cube_1))
  (Variables|Default|SetOn%20? true)
  (bind _height (Timeline|Timeline Play)
    (:Update
      (if (Variables|Default|GetOn%20?)
        (if (Variables|Default|GetRequired%20Time%20Completed%20?)
          (Utilities|FlowControl|Sequence :!label _label
            (:then_0
              (Transformation|SetRelativeLocation _cube_1 (Math|Vector|MakeVector (.x _relativelocation) (Math|Float|Lerp 5e+01 1.5e+02 _height) (.z _relativelocation)) false false))
            (:then_1
              (Transformation|SetRelativeLocation (Variables|Default|GetCube%202) (Math|Vector|MakeVector (.x _relativelocation) (* (Math|Float|Lerp 5e+01 1.5e+02 _height) -1.0) (.z _relativelocation)) false false))))
        (else
          (goto _label))))))

(fn ConstructionScript)