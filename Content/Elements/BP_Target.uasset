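; BP_Target is a one-shot shootable target that reacts to being hit by a BP_SmallBullet or BP_Laser.
; The first qualifying overlap on its static mesh notifies its Target reference with itself as source and Remove set to true.
; It then flags itself destroyed to ignore further hits and swaps a mesh material to M_TargetOff, leaving the actor in place.
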(event OnComponentBeginOverlap(StaticMesh)
  (params (OverlappedComponent :type Primitive%20Component%20Object%20Reference) (OtherActor :type Actor%20Object%20Reference) (OtherComp :type Primitive%20Component%20Object%20Reference) (OtherBodyIndex :type Integer) (bFromSweep :type Boolean) (SweepResult :type Hit%20Result%20Structure%20%28by%20ref%29))
  (if (not (Variables|Default|GetIsDestroyed))
    (Utilities|Casting|CastToBP_SmallBullet OtherActor
      (:then
        _)
      (:CastFailed
        (Utilities|Casting|CastToBP_Laser OtherActor)))
    (Default|Notify (Variables|Default|GetTarget) self true)
    (Variables|Default|SetIsDestroyed true)
    (Rendering|Material|SetMaterial (Variables|Default|GetStaticMesh) 2 "/Game/GA/PROPS/Target/M_TargetOff.M_TargetOff")))

(event EventBeginPlay
  (|CallParentFunction) ; This node is disabled and will not be called.\nDrag off pins to build functionality.
)

(event Collision|EventActorBeginOverlap
  (params (OtherActor :type Actor%20Object%20Reference)))

(event EventTick
  (params (DeltaSeconds :type Float%20%28single-precision%29)))

(fn ConstructionScript
  (|CallParentFunction))