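; Interactive sliding double door that opens on a SwitchON event and closes on SwitchOFF or when BP_Player begins overlapping its Box.
; A timeline plays forward or in reverse, driving a Lerp that slides Cube1 along Y and mirrors Cube2 to the opposite side.
; Opening movement applies only while RequiredTimeCompleted is true, a flag this graph never sets, while closing movement is unconditional.
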(event OnComponentBeginOverlap(Box)
  (params (OverlappedComponent :type Primitive%20Component%20Object%20Reference) (OtherActor :type Actor%20Object%20Reference) (OtherComp :type Primitive%20Component%20Object%20Reference) (OtherBodyIndex :type Integer) (bFromSweep :type Boolean) (SweepResult :type Hit%20Result%20Structure%20%28by%20ref%29))
  (bind _cube_1 (Variables|Default|GetCube%201))
  (bind _relativelocation (Variables|/Script/Engine.SceneComponent|GetRelativeLocation _cube_1))
  (Utilities|Casting|CastToBP_Player OtherActor)
  (Variables|Default|SetOn%20? false)
  (bind _height (Timeline|Timeline Reverse)
    (:Update
      (if (Variables|Default|GetOn%20?)
        (if (Variables|Default|GetRequired%20Time%20Completed%20?)
          (Utilities|FlowControl|Sequence :!label _label
            (:then_0
              (Transformation|SetRelativeLocation _cube_1 (Math|Vector|MakeVector (.x _relativelocation) (Math|Float|Lerp (Variables|Default|GetBase%20Y%20pos) 1.5e+02 _height) (.z _relativelocation)) false false))
            (:then_1
              (Transformation|SetRelativeLocation (Variables|Default|GetCube%202) (Math|Vector|MakeVector (.x _relativelocation) (* (Math|Float|Lerp (Variables|Default|GetBase%20Y%20pos) 1.5e+02 _height) -1.0) (.z _relativelocation)) false false))))
        (else
          (goto _label))))))

(event Custom|Switch%20OFF
  (bind _cube_1 (Variables|Default|GetCube%201))
  (bind _relativelocation (Variables|/Script/Engine.SceneComponent|GetRelativeLocation _cube_1))
  (Variables|Default|SetOn%20? false)
  (bind _height (Timeline|Timeline Reverse)
    (:Update
      (if (Variables|Default|GetOn%20?)
        (if (Variables|Default|GetRequired%20Time%20Completed%20?)
          (Utilities|FlowControl|Sequence :!label _label
            (:then_0
              (Transformation|SetRelativeLocation _cube_1 (Math|Vector|MakeVector (.x _relativelocation) (Math|Float|Lerp (Variables|Default|GetBase%20Y%20pos) 1.5e+02 _height) (.z _relativelocation)) false false))
            (:then_1
              (Transformation|SetRelativeLocation (Variables|Default|GetCube%202) (Math|Vector|MakeVector (.x _relativelocation) (* (Math|Float|Lerp (Variables|Default|GetBase%20Y%20pos) 1.5e+02 _height) -1.0) (.z _relativelocation)) false false))))
        (else
          (goto _label))))))

(event Custom|Switch%20ON
  (bind _cube_1 (Variables|Default|GetCube%201))
  (bind _relativelocation (Variables|/Script/Engine.SceneComponent|GetRelativeLocation _cube_1))
  (Variables|Default|SetOn%20? true)
  (bind _height (Timeline|Timeline Play)
    (:Update
      (if (Variables|Default|GetOn%20?)
        (if (Variables|Default|GetRequired%20Time%20Completed%20?)
          (Utilities|FlowControl|Sequence :!label _label
            (:then_0
              (Transformation|SetRelativeLocation _cube_1 (Math|Vector|MakeVector (.x _relativelocation) (Math|Float|Lerp (Variables|Default|GetBase%20Y%20pos) 1.5e+02 _height) (.z _relativelocation)) false false))
            (:then_1
              (Transformation|SetRelativeLocation (Variables|Default|GetCube%202) (Math|Vector|MakeVector (.x _relativelocation) (* (Math|Float|Lerp (Variables|Default|GetBase%20Y%20pos) 1.5e+02 _height) -1.0) (.z _relativelocation)) false false))))
        (else
          (goto _label))))))

(event EventBeginPlay
  (Variables|Default|SetBase%20Y%20pos (.y (Variables|/Script/Engine.SceneComponent|GetRelativeLocation (Variables|Default|GetCube%201)))))

(fn ConstructionScript)