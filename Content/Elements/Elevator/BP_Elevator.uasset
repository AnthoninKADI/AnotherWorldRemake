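; BP_Elevator is a multi-level elevator that carries the player and a follower between heights stored in Levels.
; Activate requires a BP_FollowerBase inside its sphere, otherwise sets the controller's AllowFollow; the console the player overlaps selects up or down.
; Move starts a Tick-driven Z interpolation timed by distance over Speed, with invisible collision enabled during travel.
; Begin sound chains into a self-respawning loop through audio-finished callbacks, ending with an arrival sound.
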(event OnComponentBeginOverlap(Sphere)
  (params (OverlappedComponent :type Primitive%20Component%20Object%20Reference) (OtherActor :type Actor%20Object%20Reference) (OtherComp :type Primitive%20Component%20Object%20Reference) (OtherBodyIndex :type Integer) (bFromSweep :type Boolean) (SweepResult :type Hit%20Result%20Structure%20%28by%20ref%29))
  (Utilities|Casting|CastToBP_FollowerBase OtherActor)
  (Variables|Default|SetFollowerOn true))

(event OnComponentEndOverlap(Sphere)
  (params (OverlappedComponent :type Primitive%20Component%20Object%20Reference) (OtherActor :type Actor%20Object%20Reference) (OtherComp :type Primitive%20Component%20Object%20Reference) (OtherBodyIndex :type Integer))
  (Utilities|Casting|CastToBP_FollowerBase OtherActor)
  (Variables|Default|SetFollowerOn false))

(event Custom|Move
  (params (From :type Float%20%28double-precision%29) (To :type Float%20%28double-precision%29))
  (Variables|Default|SetFrom From)
  (Variables|Default|SetTo To)
  (bind _output_get (Variables|Default|SetIsMoving? true))
  (bind _returnvalue (Audio|SpawnSoundatLocation "/Game/Sound/Elevator/SeparatedSounds/Elevator_Begin.Elevator_Begin" "0, 0, 0" "0, 0, 0" 1.0 1.0 0.0 0 0))
  (bind _output_get_2 (Variables|Default|SetBegin%20Elevator _returnvalue))
  (EventDispatchers|BindEventtoOnAudioFinished _output_get_2 (delegate Custom|Audio_Finished_Event))
  (Variables|Default|SetElapsedTime 0.0))

(event Custom|Audio_Finished_Event
  (if (stale Custom|Move _output_get)
    (bind _returnvalue (Audio|SpawnSoundatLocation "/Game/Sound/Elevator/SeparatedSounds/Elevator_Loop.Elevator_Loop" "0, 0, 0" "0, 0, 0" 1.0 1.0 0.0 0 0))
    (bind _output_get (Variables|Default|SetLoop%20Elevator _returnvalue))
    (EventDispatchers|BindEventtoOnAudioFinished _output_get (delegate Custom|Audio_Finished_Event))))

(event EventBeginPlay)

(event Collision|EventActorBeginOverlap
  (params (OtherActor :type Actor%20Object%20Reference)))

(event EventTick
  (params (DeltaSeconds :type Float%20%28single-precision%29))
  (bind _returnvalue (Transformation|GetActorLocation))
  (bind _from (Variables|Default|GetFrom))
  (bind _to (Variables|Default|GetTo))
  (bind _loop_elevator (Variables|Default|GetLoop%20Elevator))
  (if (Variables|Default|GetIsMoving?)
    (Variables|Default|SetElapsedTime (+ (Variables|Default|GetElapsedTime) DeltaSeconds))
    (Transformation|SetActorLocation (Math|Vector|MakeVector (.x _returnvalue) (.y _returnvalue) (Class|KismetMathLibrary|FInterpEaseinOut _from _to (/ (Variables|Default|GetElapsedTime) (/ (Math|Float|Absolute(Float) (- _from _to)) (Variables|Default|GetSpeed))) 1.0)) false false)
    (if (>= (/ (Variables|Default|GetElapsedTime) (/ (Math|Float|Absolute(Float) (- _from _to)) (Variables|Default|GetSpeed))) 1.0)
      (Variables|Default|SetIsMoving? false)
      (Utilities|IsValid _loop_elevator
        (:Is%20Valid
          (Audio|Components|Audio|Stop _loop_elevator)
          (Components|DestroyComponent _loop_elevator)
          (Audio|PlaySoundatLocation "/Game/Sound/Elevator/SeparatedSounds/Elevator_End.Elevator_End" "0, 0, 0" "0, 0, 0" 1.0 1.0 0.0 0 0 0 0)
          (Collision|SetCollisionEnabled (Variables|Default|GetInvisible%20Collision01) "NoCollision"))))))

(fn ConstructionScript)

(fn Activate
  (bind _returnvalue (Game|GetPlayerCharacter 0))
  (bind _elevator (Variables|Default|GetElevator))
  (bind _returnvalue_2 (Transformation|GetWorldLocation _elevator))
  (if (not (Variables|Default|GetIsMoving?))
    (if (Variables|Default|GetFollowerOn)
      (Audio|PlaySoundatLocation "/Game/Sound/Buttons/Button_Elevator.Button_Elevator" "0, 0, 0" "0, 0, 0" 1.0 1.0 0.0 0 0 0 0)
      (if (Collision|IsOverlappingActor (Variables|Default|GetConsoleCollision) _returnvalue :!class /Script/Engine.PrimitiveComponent)
        (if (< (Variables|Default|GetCurrLevel) (Utilities|Array|Length (Variables|Default|GetLevels)))
          (CallFunction|Move (.z _returnvalue_2) (Utilities|Array|Get(acopy) (Variables|Default|GetLevels) (Variables|Default|GetCurrLevel)))
          (Variables|Default|SetCurrLevel (+ (Variables|Default|GetCurrLevel) 1))
          (Collision|SetCollisionEnabled (Variables|Default|GetInvisible%20Collision01) "QueryAndPhysics" :!label _label))
        (elif (Collision|IsOverlappingActor (Variables|Default|GetConsoleCollision1) _returnvalue :!class /Script/Engine.PrimitiveComponent)
          (if (> (Variables|Default|GetCurrLevel) 1)
            (CallFunction|Move (.z _returnvalue_2) (Utilities|Array|Get(acopy) (Variables|Default|GetLevels) (- (Variables|Default|GetCurrLevel) 2)))
            (Variables|Default|SetCurrLevel (- (Variables|Default|GetCurrLevel) 1))
            (goto _label))))
      (else
        (Variables|/Game/_GameManager/BP_PlayerController.BP_PlayerController_C|SetAllow%20Follow? (.AsBP%20Player%20Controller (Utilities|Casting|CastToBP_PlayerController (Game|GetPlayerController 0))) true)))))