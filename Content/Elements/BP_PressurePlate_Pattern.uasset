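; Pressure plate that lowers a target object between two hard-coded world positions while occupied, tinting its base green on entry and red on exit.
; An overlap counter drives a Timeline forward while positive and in reverse at zero, with a short delay on entry only.
; DoOnce nodes limit the camera reveal to one showing, blending to a Camera on the first update and back to the player when the Timeline finishes.
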(event OnComponentBeginOverlap(Trigger)
  (params (OverlappedComponent :type Primitive%20Component%20Object%20Reference) (OtherActor :type Actor%20Object%20Reference) (OtherComp :type Primitive%20Component%20Object%20Reference) (OtherBodyIndex :type Integer) (bFromSweep :type Boolean) (SweepResult :type Hit%20Result%20Structure%20%28by%20ref%29))
  (bind _activatorcount (Variables|Default|GetActivatorCount))
  (Rendering|Material|SetMaterial (Variables|Default|GetBase) 1 (Variables|mat|GetGreen))
  ;[1 1 1] Keeps track of the total amount of people on the plate, and only sends positive trigger when at least one is on
  (Math|Integer|IncrementInt _activatorcount
    (:%20%20
      (Utilities|FlowControl|Delay 0.4)
      (if (> _activatorcount 0)
        (bind _newtrack_0 (Timeline|Timeline Play)
          (:Update
            (Transformation|SetActorLocation (Variables|Default|GetObjectToMove) (Math|Vector|Lerp(Vector) "5020.000000,-1380.000000,525.000000" "5020.000000,-1380.000000,425.000000" _newtrack_0) false false)
            (Utilities|FlowControl|DoOnce false
              (:Completed
                (Game|Player|SetViewTargetwithBlend (Game|GetPlayerController 0) (Variables|Default|GetCamera) 0.5 "VTBlend_PreBlended" 0.0 false))))
          (:Finished
            (Utilities|FlowControl|DoOnce false
              (:Completed
                (Game|Player|SetViewTargetwithBlend (Game|GetPlayerController 0) (Game|GetPlayerCharacter 0) 0.5 "VTBlend_PreBlended" 0.0 false)))))
        (else
          (Timeline|Timeline Reverse))))))

(event OnComponentEndOverlap(Trigger)
  (params (OverlappedComponent :type Primitive%20Component%20Object%20Reference) (OtherActor :type Actor%20Object%20Reference) (OtherComp :type Primitive%20Component%20Object%20Reference) (OtherBodyIndex :type Integer))
  (bind _activatorcount (Variables|Default|GetActivatorCount))
  (Rendering|Material|SetMaterial (Variables|Default|GetBase) 1 (Variables|mat|GetRed))
  ;[1 1 1] Keeps track of the total amount of people on the plate, and only sends positive trigger when at least one is on
  (Math|Integer|DecrementInt _activatorcount
    (:%20%20
      (if (> _activatorcount 0)
        (bind _newtrack_0 (Timeline|Timeline Play)
          (:Update
            (Transformation|SetActorLocation (Variables|Default|GetObjectToMove) (Math|Vector|Lerp(Vector) "5020.000000,-1380.000000,525.000000" "5020.000000,-1380.000000,425.000000" _newtrack_0) false false)
            (Utilities|FlowControl|DoOnce false
              (:Completed
                (Game|Player|SetViewTargetwithBlend (Game|GetPlayerController 0) (Variables|Default|GetCamera) 0.5 "VTBlend_PreBlended" 0.0 false))))
          (:Finished
            (Utilities|FlowControl|DoOnce false
              (:Completed
                (Game|Player|SetViewTargetwithBlend (Game|GetPlayerController 0) (Game|GetPlayerCharacter 0) 0.5 "VTBlend_PreBlended" 0.0 false)))))
        (else
          (Timeline|Timeline Reverse))))))

(fn ConstructionScript)