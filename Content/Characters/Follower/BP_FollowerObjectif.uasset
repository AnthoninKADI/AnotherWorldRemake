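; BP_FollowerObjectif is a trigger objective that brings enemies into play when a follower reaches it.
; Overlap by a component tagged Follower starts a delay, then teleports each EnemyList entry to the matching SpawnPointList location by shared index.
; It then waits for the InteractionTime read from a BP_FollowerBase actor found in the level and destroys itself.
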(event OnComponentBeginOverlap(Box)
  (params (OverlappedComponent :type Primitive%20Component%20Object%20Reference) (OtherActor :type Actor%20Object%20Reference) (OtherComp :type Primitive%20Component%20Object%20Reference) (OtherBodyIndex :type Integer) (bFromSweep :type Boolean) (SweepResult :type Hit%20Result%20Structure%20%28by%20ref%29))
  (if (Components|ComponentHasTag OtherComp "Follower")
    (Utilities|FlowControl|Delay (Variables|Default|GetSpawnEnemyTime))
    (for (_array_element _array_index) (Variables|Default|GetSpawnPointList)
      (Transformation|Teleport (Utilities|Array|Get(acopy) (Variables|Default|GetEnemyList) _array_index) (Transformation|GetWorldLocation (Variables|/Game/Characters/Enemy/BP_EnemySpawnPoint.BP_EnemySpawnPoint_C|GetDefaultSceneRoot _array_element)) "0, 0, 0"))
    (bind _returnvalue (Actor|GetActorOfClass "/Game/Characters/Follower/BP_FollowerBase.BP_FollowerBase_C"))
    (Utilities|FlowControl|Delay (Variables|/Game/Characters/Follower/BP_FollowerBase.BP_FollowerBase_C|GetInteractionTime _returnvalue))
    (Actor|DestroyActor)))

(fn ConstructionScript)