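; BP_Trigger_Target is a shootable target trigger that breaks when hit by a small bullet or laser.
; It flags itself as a target before running the parent's BeginPlay.
; The first valid box overlap notifies its linked Target with a remove request and sets IsDestroyed to block further hits.
; It then swaps to a broken mesh and spawns attached Niagara sparks offset and rotated from the mesh's relative transform.
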(event OnComponentBeginOverlap(Box)
  (params (OverlappedComponent :type Primitive%20Component%20Object%20Reference) (OtherActor :type Actor%20Object%20Reference) (OtherComp :type Primitive%20Component%20Object%20Reference) (OtherBodyIndex :type Integer) (bFromSweep :type Boolean) (SweepResult :type Hit%20Result%20Structure%20%28by%20ref%29))
  (bind _staticmesh (Variables|Default|GetStaticMesh))
  (bind _relativerotation (Variables|/Script/Engine.SceneComponent|GetRelativeRotation _staticmesh))
  (if (not (Variables|Default|GetIsDestroyed))
    (Utilities|Casting|CastToBP_SmallBullet OtherActor
      (:then
        _)
      (:CastFailed
        (Utilities|Casting|CastToBP_Laser OtherActor)))
    (Default|Notify (Variables|Default|GetTarget) self true)
    (Variables|Default|SetIsDestroyed true)
    (Components|StaticMesh|SetStaticMesh (Variables|Default|GetStaticMesh) "/Game/GA/PROPS/Target/SM_Targets_SM_Target_Broken.SM_Targets_SM_Target_Broken")
    (Niagara|SpawnSystemAttached "/Game/GA/VFX/NS/Enviro/NS_BreakSparks.NS_BreakSparks" _staticmesh "" (+ (Variables|/Script/Engine.SceneComponent|GetRelativeLocation _staticmesh) "10.000000,10.000000,10.000000") (Math|Rotator|MakeRotator (.roll _relativerotation) (+ (.pitch _relativerotation) 9e+01) (.yaw _relativerotation)) "KeepRelativeOffset" false)))

(event EventBeginPlay
  (Variables|Default|SetIsTarget? true)
  (|CallParentFunction))

(fn ConstructionScript
  (|CallParentFunction))