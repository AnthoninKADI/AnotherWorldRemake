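; BP_Weapon is the player's gun actor, providing a hold-to-charge shot and a deployable shield.
; Shoot builds charge with particles, then on release fires BP_Laser when fully charged or BP_SmallBullet otherwise, with camera-facing rotation, feedback and recoil delay.
; Tick runs cooldown and shield charge, spawning BP_FullShield when released fully charged and replacing the oldest at MaxShield.
; CastShield jumps straight into that spawn logic, bypassing the charge check.
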(event Custom|Cast%20Shield
  (bind _ownercharacter (Variables|Default|GetOwnerCharacter))
  (bind _shieldarray (Variables|Shield|GetshieldArray))
  (bind _shieldrelativespawnposition (Variables|Shield|GetShieldRelativeSpawnPosition))
  (bind _returnvalue (Transformation|GetActorTransform _ownercharacter))
  (bind _returnvalue_2 (Math|Vector|RotateVector _shieldrelativespawnposition (.rotation _returnvalue)))
  (bind _returnvalue_3 (+ _returnvalue_2 (.location _returnvalue)))
  ;[0.121 1 0.9203] Spawn shield depending on timh hold
  (if (== (Utilities|Array|Length _shieldarray) (Variables|Shield|GetmaxShield))
    (Actor|DestroyActor (Utilities|Array|Get(acopy) _shieldarray))
    (Utilities|Array|RemoveIndex _shieldarray))
  (bind _returnvalue_4 (Game|SpawnActorfromClass "/Game/Characters/Weapon/BP_FullShield.BP_FullShield_C" (Math|Transform|MakeTransform _returnvalue_3 (.rotation _returnvalue) (.scale _returnvalue)) "Undefined" "MultiplyWithRoot" 0 0))
  (Audio|PlaySoundatLocation 0 _returnvalue_3 "0, 0, 0" 1.0 1.0 0.0 0 0 0 0)
  (Variables|/Game/Characters/Weapon/BP_FullShield.BP_FullShield_C|SetOwningWeapon _returnvalue_4 self)
  (Utilities|Array|Add (Variables|Shield|GetshieldArray) _returnvalue_4)
  (Variables|Shield|SetCurrent%20ShieldLevel 0.0)
  (Components|DestroyComponent (Variables|Shield|GetShieldParticle))
  (Variables|Default|SetParticleSpawnedShield false))

(event Custom|Shoot
  (params (Active :type Boolean) (DeltaSecond :type Float%20%28double-precision%29) (TargetPoint :type Vector))
  (bind _returnvalue (Game|GetPlayerController 0))
  (bind _returnvalue_2 (Transformation|GetActorLocation))
  (bind _returnvalue_3 (Game|GetPlayerController 0))
  (bind _gun (Variables|Default|GetGUN))
  (bind _gun_2 (Variables|Default|GetGUN))
  (bind _gun_3 (Variables|Default|GetGUN))
  (bind _returnvalue_4 (Transformation|GetSocketLocation _gun_3 "GunShoot"))
  (bind _returnvalue_5 (Transformation|GetSocketLocation _gun_2 "GunShoot"))
  (bind _asbp_player_controller (Utilities|Casting|CastToBP_PlayerController _returnvalue_3))
  (bind _asbp_player_controller_2 (Utilities|Casting|CastToBP_PlayerController _returnvalue))
  (bind _returnvalue_6 (Math|Rotator|FindLookatRotation _returnvalue_4 TargetPoint))
  (if Active
    (if (== (Variables|Laser|GetLaserCurrentLevel) 0.0)
      (Game|Feedback|ClientPlayForceFeedback (Game|GetPlayerController 0) "/Game/Elements/ForceFeedbacks/FFE_EnergyCrescendo.FFE_EnergyCrescendo" "None" false false false))
    ;[1 0.04393 0.2242] Select Laser depending on the time holding
    (if (Variables|Default|GetParticleSpawnedLaser)
      _
      (else
        (bind _returnvalue_7 (Niagara|SpawnSystemAttached "/Game/GA/VFX/NS/Character/NS_LongBeam_Charge_Particles.NS_LongBeam_Charge_Particles" (Variables|Default|GetGUN) "GunShoot" "0, 0, 0" "0, 0, 0" "KeepRelativeOffset" true))
        (bind _returnvalue_8 (AddComponent|AddNiagaraComponent false))
        (Class|NiagaraComponent|AdvanceSimulation _returnvalue_8 10 (* (stale EventTick DeltaSeconds) 1e+01))
        (Transformation|AttachComponentToComponent _returnvalue_8 (Variables|Default|GetGUN) "GunShoot" "KeepRelative" "KeepRelative" "KeepRelative" true)
        (Audio|SpawnSoundAttached 0 0 "None" "0, 0, 0" "0, 0, 0" "KeepRelativeOffset" false 1.0 1.0 0.0 0 0)
        (Variables|Default|SetParticleSpawnedLaser true)))
    (Variables|Laser|SetLaserCurrentLevel (+ (* DeltaSecond (Variables|Laser|GetLaserIncreaseRate)) (Variables|Laser|GetLaserCurrentLevel)))
    (else
      ;[0.35 0.45 1] Rotate Player Forward To Camera Forward
      (bind _asbp_player (Utilities|Casting|CastToBP_Player (Variables|Default|GetOwnerCharacter))
        (:then
          (Transformation|SetActorRelativeRotation _asbp_player (Math|Rotator|MakeRotator (.Roll (Math|Rotator|BreakRotator (Transformation|GetActorRotation _asbp_player))) (.Pitch (Math|Rotator|BreakRotator (Transformation|GetActorRotation _asbp_player))) (.yaw (Variables|/Script/Engine.SceneComponent|GetRelativeRotation (Variables|/Script/Engine.PlayerCameraManager|GetTransformComponent (Game|GetPlayerCameraManager 0))))) true)
          (if (Variables|/Game/_GameManager/BP_PlayerController.BP_PlayerController_C|GetIs%20Aiming%20? _asbp_player_controller_2)
            (Variables|Default|SetwasAiming? true)
            (else
              (Class|Image|SetBrush (Variables|/Game/UI/W_AimPoint.W_AimPoint_C|GetImage_76 (Variables|/Game/_GameManager/BP_PlayerController.BP_PlayerController_C|GetAimPoint _asbp_player_controller_2)) (Utilities|Struct|MakeSlateBrush "Image" "NoTile" "NoMirror" "(X=32.000000,Y=32.000000)" "(Left=0.000000,Top=0.000000,Right=0.000000,Bottom=0.000000)" "(SpecifiedColor=(R=1.000000,G=1.000000,B=1.000000,A=1.000000),ColorUseRule=UseColor_Specified)" "(CornerRadii=(X=0.000000,Y=0.000000,Z=0.000000,W=1.000000),Color=(SpecifiedColor=(R=0.000000,G=0.000000,B=0.000000,A=0.000000),ColorUseRule=UseColor_Specified),Width=0.000000,RoundingType=HalfHeightRadius,bUseBrushTransparency=False)" "/Game/GA/UI/UI_Cursor_Spread.UI_Cursor_Spread"))
              (Variables|/Game/_GameManager/BP_PlayerController.BP_PlayerController_C|SetIs%20Aiming%20? _asbp_player_controller_2 true)
              (Utilities|FlowControl|Delay 0.2))))
        (:CastFailed
          _))
      (Variables|Default|SetCooldown (Variables|Default|GetRecoilDuration))
      (if (>= (Variables|Laser|GetLaserCurrentLevel) 1e+02)
        (bind _returnvalue_9 (Game|SpawnActorfromClass "/Game/Characters/Weapon/BP_Laser.BP_Laser_C" (Math|Transform|MakeTransform _returnvalue_5 _returnvalue_6 "1.000000,1.000000,1.000000") "Undefined" "MultiplyWithRoot" 0 0 0))
        (Niagara|SpawnSystemAttached "/Game/GA/VFX/NS/Character/NS_LongBeam_MuzzleFlash.NS_LongBeam_MuzzleFlash" _gun "GunShoot" "0, 0, 0" "0, 0, 0" "KeepRelativeOffset" false)
        (Game|Feedback|ClientPlayForceFeedback (Game|GetPlayerController 0) "/Game/Elements/ForceFeedbacks/FFE_Shoot.FFE_Shoot" "None" false false false)
        (Audio|PlaySoundatLocation 0 _returnvalue_2 "0, 0, 0" 1.0 1.0 0.0 0 0 0 0)
        (Variables|/Game/Characters/Weapon/BP_Laser.BP_Laser_C|SetOwnerCharacter _returnvalue_9 (Variables|Default|GetOwnerCharacter))
        (Variables|Laser|SetLaserCurrentLevel 0.0)
        (else
          (bind _returnvalue_10 (Game|SpawnActorfromClass "/Game/Characters/Weapon/BP_SmallBullet.BP_SmallBullet_C" (Math|Transform|MakeTransform _returnvalue_5 _returnvalue_6 "1.000000,1.000000,1.000000") "Undefined" "MultiplyWithRoot" 0 0))
          (Niagara|SpawnSystemAttached "/Game/GA/VFX/NS/Character/NS_ShortBeam_MuzzleFlash.NS_ShortBeam_MuzzleFlash" _gun "GunShoot" "0, 0, 0" "0, 0, 0" "KeepRelativeOffset" false)
          (Game|Feedback|ClientPlayForceFeedback (Game|GetPlayerController 0) "/Game/Elements/ForceFeedbacks/FFE_Shoot.FFE_Shoot" "None" false false false)
          (Audio|PlaySoundatLocation 0 _returnvalue_2 "0, 0, 0" 1.0 1.0 0.0 0 0 0 0)
          (Variables|/Game/Characters/Weapon/BP_SmallBullet.BP_SmallBullet_C|SetOwnerCharacter _returnvalue_10 (Variables|Default|GetOwnerCharacter))
          (Variables|Laser|SetLaserCurrentLevel 0.0)))
      (Variables|Default|SetParticleSpawnedLaser false)
      (Utilities|FlowControl|Delay (Variables|Default|GetRecoilDuration))
      (Variables|Default|SetShooting? false)
      (Class|Image|SetBrush (Variables|/Game/UI/W_AimPoint.W_AimPoint_C|GetImage_76 (Variables|/Game/_GameManager/BP_PlayerController.BP_PlayerController_C|GetAimPoint _asbp_player_controller)) (Utilities|Struct|MakeSlateBrush "Image" "NoTile" "NoMirror" "(X=32.000000,Y=32.000000)" "(Left=0.000000,Top=0.000000,Right=0.000000,Bottom=0.000000)" (Utilities|Struct|MakeSlateColor "(R=1.000000,G=1.000000,B=1.000000,A=0.000000)" "UseColor_Specified") "(CornerRadii=(X=0.000000,Y=0.000000,Z=0.000000,W=1.000000),Color=(SpecifiedColor=(R=0.000000,G=0.000000,B=0.000000,A=0.000000),ColorUseRule=UseColor_Specified),Width=0.000000,RoundingType=HalfHeightRadius,bUseBrushTransparency=False)" 0))
      (if (Variables|Default|GetwasAiming?)
        _
        (else
          (Variables|/Game/_GameManager/BP_PlayerController.BP_PlayerController_C|SetIs%20Aiming%20? _asbp_player_controller false)))
      (Variables|Default|SetwasAiming? false)
      (Utilities|IsValid _returnvalue_8
        (:Is%20Valid
          (Components|DestroyComponent _returnvalue_8))
        (:Is%20Not%20Valid
          _))
      (Utilities|IsValid _returnvalue_7
        (:Is%20Valid
          (Components|DestroyComponent _returnvalue_7))))))

(event EventTick
  (params (DeltaSeconds :type Float%20%28single-precision%29))
  (bind _ownercharacter (Variables|Default|GetOwnerCharacter))
  (bind _shieldarray (Variables|Shield|GetshieldArray))
  (bind _shieldrelativespawnposition (Variables|Shield|GetShieldRelativeSpawnPosition))
  (bind _returnvalue (Transformation|GetActorTransform _ownercharacter))
  (bind _returnvalue_2 (Math|Vector|RotateVector _shieldrelativespawnposition (.rotation _returnvalue)))
  (bind _returnvalue_3 (+ _returnvalue_2 (.location _returnvalue)))
  ;[0.121 1 0.9203] Spawn shield depending on timh hold
  (Development|PrintString (Utilities|String|ToString(Boolean) (Variables|Default|GetShooting?)) true true "(R=0.000000,G=1.000000,B=1.000000,A=1.000000)" 0.0)
  (Utilities|FlowControl|Sequence
    (:then_0
      (if (Variables|Shield|GetShieldIsActive)
        (if (Variables|Default|GetParticleSpawnedShield)
          _
          (else
            (bind _returnvalue_4 (AddComponent|AddNiagaraComponent false))
            (bind _output_get (Variables|Shield|SetShieldParticle _returnvalue_4))
            (Class|NiagaraComponent|AdvanceSimulation _returnvalue_4 10 (* DeltaSeconds 1e+01))
            (Transformation|AttachComponentToComponent _output_get (Variables|Default|GetGUN) "GunShoot" "KeepRelative" "KeepRelative" "KeepRelative" true)
            (Audio|SpawnSoundAttached 0 0 "None" "0, 0, 0" "0, 0, 0" "KeepRelativeOffset" false 1.0 1.0 0.0 0 0)
            (Variables|Default|SetParticleSpawnedShield true)))
        (Variables|Shield|SetCurrent%20ShieldLevel (+ (Variables|Shield|GetCurrent%20ShieldLevel) (* DeltaSeconds (Variables|Shield|GetShieldIncreaseRate))))
        (else
          (bind _output_get_2 (Variables|Shield|SetCurrent%20ShieldLevel (Math|Float|Clamp(Float) (- (Variables|Shield|GetCurrent%20ShieldLevel) (* DeltaSeconds (Variables|Shield|GetShieldDecreaseRate))) 0.0 1.2e+02)))
          (if (>= _output_get_2 1e+02)
            ;[0.35 0.45 1] Rotate Player Forward To Camera Forward
            (bind _asbp_player (Utilities|Casting|CastToBP_Player (Variables|Default|GetOwnerCharacter))
              (:then
                (Transformation|SetActorRelativeRotation _asbp_player (Math|Rotator|MakeRotator (.Roll (Math|Rotator|BreakRotator (Transformation|GetActorRotation _asbp_player))) (.Pitch (Math|Rotator|BreakRotator (Transformation|GetActorRotation _asbp_player))) (.yaw (Variables|/Script/Engine.SceneComponent|GetRelativeRotation (Variables|/Script/Engine.PlayerCameraManager|GetTransformComponent (Game|GetPlayerCameraManager 0))))) true))
              (:CastFailed
                _))
            (if (== (Utilities|Array|Length _shieldarray) (Variables|Shield|GetmaxShield))
              (Actor|DestroyActor (Utilities|Array|Get(acopy) _shieldarray))
              (Utilities|Array|RemoveIndex _shieldarray))
            (bind _returnvalue_5 (Game|SpawnActorfromClass "/Game/Characters/Weapon/BP_FullShield.BP_FullShield_C" (Math|Transform|MakeTransform _returnvalue_3 (.rotation _returnvalue) (.scale _returnvalue)) "Undefined" "MultiplyWithRoot" 0 0))
            (Audio|PlaySoundatLocation 0 _returnvalue_3 "0, 0, 0" 1.0 1.0 0.0 0 0 0 0)
            (Variables|/Game/Characters/Weapon/BP_FullShield.BP_FullShield_C|SetOwningWeapon _returnvalue_5 self)
            (Utilities|Array|Add (Variables|Shield|GetshieldArray) _returnvalue_5)
            (Variables|Shield|SetCurrent%20ShieldLevel 0.0)
            (Components|DestroyComponent (Variables|Shield|GetShieldParticle))
            (Variables|Default|SetParticleSpawnedShield false)
            (else
              (Utilities|IsValid (Variables|Shield|GetShieldParticle)
                (:Is%20Valid
                  (Components|DestroyComponent (Variables|Shield|GetShieldParticle))
                  (Variables|Default|SetParticleSpawnedShield false))))))))
    (:then_1
      (if (> (Variables|Default|GetCooldown) 0.0)
        (Variables|Default|SetCooldown (- (Variables|Default|GetCooldown) DeltaSeconds))))))

(fn ConstructionScript)