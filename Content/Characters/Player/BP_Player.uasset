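; BP_Player is the player character, handling movement speeds, starting health, weapon spawning and death.
; BeginPlay spawns a test BP_Weapon at the camera, sets itself as owner and passes it to BP_PlayerController.
; Healing raises HealthComponent health on a self-referencing timer while out of combat and below maximum.
; HitProjectile subtracts damage and, at zero health, pauses, shows W_GameOver and switches to UI input.
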(event Custom|Healing
  (bind _healthcomponent (Variables|Default|GetHealthComponent))
  ;[0.5365 1 0.2927] Heal System
  (if (and (!= (Variables|Default|GetInCombat) true) (< (Variables|/Script/AnotherWorldRemake.HealthComponent|GetCurrent _healthcomponent) (Variables|/Script/AnotherWorldRemake.HealthComponent|GetMaxHealth _healthcomponent)))
    (Utilities|Time|SetTimerbyEvent (delegate Custom|Healing) 2.0 (and (!= (Variables|Default|GetInCombat) true) (< (Variables|/Script/AnotherWorldRemake.HealthComponent|GetCurrent _healthcomponent) (Variables|/Script/AnotherWorldRemake.HealthComponent|GetMaxHealth _healthcomponent))))
    (Variables|/Script/AnotherWorldRemake.HealthComponent|SetCurrent _healthcomponent (+ (Variables|/Script/AnotherWorldRemake.HealthComponent|GetCurrent _healthcomponent) 10))))

(event EventHitProjectile
  (params (Damage :type Integer) (Projectile :type Actor%20Object%20Reference))
  (bind _returnvalue (PlayerController|LocalPlayerSubsystems|GetEnhancedInputLocalPlayerSubsystem))
  (bind _healthcomponent (Variables|Default|GetHealthComponent))
  (bind _output_get (Variables|/Script/AnotherWorldRemake.HealthComponent|SetCurrent _healthcomponent (- (Variables|/Script/AnotherWorldRemake.HealthComponent|GetCurrent _healthcomponent) Damage)))
  ;[1 1 1] if true, lose game
  (if (<= _output_get 0)
    ;[1 0 0] Game Over Screen
    (Game|SetGamePaused true)
    (bind _returnvalue_2 (UserInterface|CreateWidget "/Game/UI/W_GameOver.W_GameOver_C"))
    (UserInterface|Viewport|AddtoViewport _returnvalue_2 0)
    (Input|SetInputModeUIOnly 0 _returnvalue_2 "DoNotLock" false)
    (Input|RemoveMappingContext _returnvalue "/Game/_GameManager/Input/IMC_Default.IMC_Default" "(bIgnoreAllPressedKeysUntilRelease=True,bForceImmediately=False)")
    (Input|AddMappingContext _returnvalue "/Game/_GameManager/Input/IMC_UI.IMC_UI" 0 "(bIgnoreAllPressedKeysUntilRelease=True,bForceImmediately=False)")))

(event EventBeginPlay
  (bind _charactermovement (Variables|Character|GetCharacterMovement))
  (Variables|/Script/Engine.CharacterMovementComponent|SetMaxWalkSpeed _charactermovement (Variables|Default|GetMaxWalkSpeed))
  (Variables|/Script/Engine.CharacterMovementComponent|SetMaxWalkSpeedCrouched _charactermovement (Variables|Default|GetMaxCrouchSpeed))
  (Variables|/Script/AnotherWorldRemake.HealthComponent|SetCurrent (Variables|Default|GetHealthComponent) 50)
  ;[1 1 1] For testing purpose
  (bind _returnvalue (Game|SpawnActorfromClass "/Game/Characters/Weapon/BP_Weapon.BP_Weapon_C" (Transformation|GetWorldTransform (Variables|Default|GetCamera)) "Undefined" "MultiplyWithRoot" 0 0))
  (Variables|/Game/Characters/Weapon/BP_Weapon.BP_Weapon_C|SetOwnerCharacter _returnvalue self)
  (Variables|/Game/_GameManager/BP_PlayerController.BP_PlayerController_C|SetWeapon (.AsBP%20Player%20Controller (Utilities|Casting|CastToBP_PlayerController (Game|GetPlayerController 0))) _returnvalue)
  (Actor|GetActorOfClass "/Game/Characters/Follower/BP_FollowerBase.BP_FollowerBase_C"))

(fn ConstructionScript)