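; Trigger volume Blueprint that sets off a bat flyby effect when a Character enters its box.
; On overlap, it activates the particle component of every entry in the ParticlesToTrigger array and plays the BatsFlyby and BatFlybySqueak sounds.
; Box collision is disabled inside that same loop, so the effect fires once, and an empty array leaves the trigger live and silent.
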(event OnComponentBeginOverlap(Box)
  (params (OverlappedComponent :type Primitive%20Component%20Object%20Reference) (OtherActor :type Actor%20Object%20Reference) (OtherComp :type Primitive%20Component%20Object%20Reference) (OtherBodyIndex :type Integer) (bFromSweep :type Boolean) (SweepResult :type Hit%20Result%20Structure%20%28by%20ref%29))
  (Utilities|Casting|CastToCharacter OtherActor)
  (if (> (Utilities|Array|Length (Variables|Default|GetParticlesToTrigger)) 0)
    (for _array_element (Variables|Default|GetParticlesToTrigger)
      (Components|Activation|Activate (Variables|/Script/Engine.Emitter|GetParticleSystemComponent _array_element) false)
      (Collision|SetCollisionEnabled (Variables|Default|GetBox) "NoCollision")
      (Audio|Components|Audio|Play (Variables|Default|GetBats_Flyby) 0.0)
      (Audio|Components|Audio|Play (Variables|Default|GetBat_Flyby_Squeak) 0.0))))

(fn ConstructionScript)