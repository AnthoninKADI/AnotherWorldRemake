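; Activatable door or bridge that opens when its set of pending triggers is empty and can also act as a proximity sensor for players and followers.
; Trigger sources add or remove themselves through Notify, and CheckActivation calls Activate or Deactivate, playing sounds and switching state.
; After a retriggerable delay, a Timeline either slides two door halves apart or toggles bridge and fence visibility, collision and material-collection fade.
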(event OnComponentEndOverlap(Overlap)
  (params (OverlappedComponent :type Primitive%20Component%20Object%20Reference) (OtherActor :type Actor%20Object%20Reference) (OtherComp :type Primitive%20Component%20Object%20Reference) (OtherBodyIndex :type Integer))
  (bind _overlap (Variables|Default|GetOverlap))
  (Utilities|Casting|CastToPawn OtherActor) ; ignore lasers
  (if (Variables|Default|GetProximitySensor)
    (if (and (== (Utilities|Array|Length (Collision|GetOverlappingActors _overlap "/Game/Characters/Player/BP_Player.BP_Player_C" :!class /Script/Engine.PrimitiveComponent)) 0) (== (Utilities|Array|Length (Collision|GetOverlappingActors _overlap "/Game/Characters/Follower/BP_FollowerBase.BP_FollowerBase_C" :!class /Script/Engine.PrimitiveComponent)) 0))
      (CallFunction|Deactivate :!label _label))
    (else
      (Utilities|Casting|CastToBP_FollowerBase OtherActor)
      (bind _result (Utilities|Set|ToArray (Variables|Default|GetTriggers)))
      (if (or (Variables|/Game/Elements/BP_TriggerActor.BP_TriggerActor_C|GetShouldStay? (Utilities|Array|Get(acopy) _result)) (Variables|Default|GetOneWay?))
        (goto _label)))))

(event OnComponentBeginOverlap(Overlap)
  (params (OverlappedComponent :type Primitive%20Component%20Object%20Reference) (OtherActor :type Actor%20Object%20Reference) (OtherComp :type Primitive%20Component%20Object%20Reference) (OtherBodyIndex :type Integer) (bFromSweep :type Boolean) (SweepResult :type Hit%20Result%20Structure%20%28by%20ref%29))
  (Utilities|Casting|CastToBP_Player OtherActor
    (:then
      _)
    (:CastFailed
      (Utilities|Casting|CastToBP_FollowerBase OtherActor)))
  (if (Variables|Default|GetProximitySensor)
    (CallFunction|CheckActivation)))

(event Custom|Switch%20OFF
  (bind _cube_2_to_move (Variables|Refs|GetCube%202%20To%20Move))
  (bind _base_y_pos (Variables|BasePos|GetBase%20Y%20pos))
  (bind _triggered_on_sound (Variables|SFX|GetTriggered%20On%20Sound))
  (bind _cube_1_to_move (Variables|Refs|GetCube%201%20To%20Move))
  (bind _relativelocation (Variables|/Script/Engine.SceneComponent|GetRelativeLocation _cube_1_to_move))
  (bind _relativelocation_2 (Variables|/Script/Engine.SceneComponent|GetRelativeLocation _cube_2_to_move))
  (if (Variables|Default|GetProximitySensor)
    (Utilities|IsValid _triggered_on_sound
      (:Is%20Valid
        (Audio|PlaySoundatLocation _triggered_on_sound (Transformation|GetWorldLocation (Variables|Default|GetMainMesh)) "0, 0, 0" 1.0 1.0 0.0 0 0 0 0))
      (:Is%20Not%20Valid
        _)))
  (Variables|Default|SetOn? false)
  (bind _height (Timeline|Timeline Reverse)
    (:Update
      (if (Variables|Default|GetIsBridge?)
        (if (Variables|Default|GetOn?)
          ;[0 1 1] Bridge
          ;;[0.2 1 0.2] On
          (Utilities|FlowControl|Sequence
            (:then_0
              (bind _cube_1_to_move_2 (Variables|Refs|GetCube%201%20To%20Move)
                (:then
                  (Rendering|SetVisibility _cube_1_to_move_2 true false)
                  (bind _cube_1_to_move_3 (Variables|Refs|GetCube%201%20To%20Move)
                    (:then
                      (Collision|SetCollisionEnabled _cube_1_to_move_3 "QueryAndPhysics"))
                    (:else)))
                (:else)))
            (:then_1
              (bind _front_fence_ref (Variables|Refs|GetFront%20Fence%20Ref)
                (:then
                  (Rendering|SetVisibility _front_fence_ref false false)
                  (bind _front_fence_ref_2 (Variables|Refs|GetFront%20Fence%20Ref)
                    (:then
                      (Collision|SetCollisionEnabled _front_fence_ref_2 "NoCollision"))
                    (:else)))
                (:else)))
            (:then_2
              (bind _back_fence_ref (Variables|Refs|GetBack%20Fence%20Ref)
                (:then
                  (Rendering|SetVisibility _back_fence_ref false false)
                  (bind _back_fence_ref_2 (Variables|Refs|GetBack%20Fence%20Ref)
                    (:then
                      (Collision|SetCollisionEnabled _back_fence_ref_2 "NoCollision"))
                    (:else)))
                (:else)))
            (:then_3
              (bind _r_fence_ref (Variables|Refs|GetR%20Fence%20Ref)
                (:then
                  (Rendering|SetVisibility _r_fence_ref true false)
                  (bind _r_fence_ref_2 (Variables|Refs|GetR%20Fence%20Ref)
                    (:then
                      (Collision|SetCollisionEnabled _r_fence_ref_2 "QueryAndPhysics"))
                    (:else)))
                (:else)))
            (:then_4
              (bind _l_fence_ref (Variables|Refs|GetL%20Fence%20Ref)
                (:then
                  (Rendering|SetVisibility _l_fence_ref true false)
                  (bind _l_fence_ref_2 (Variables|Refs|GetL%20Fence%20Ref)
                    (:then
                      (Collision|SetCollisionEnabled _l_fence_ref_2 "QueryAndPhysics"))
                    (:else)))
                (:else))))
          (Rendering|Material|SetScalarParameterValue "/Game/Elements/Interactibles(Loris)/MP_FadeParam.MP_FadeParam" "Bridge Fade" 1.0 :!class /Script/Engine.KismetMaterialLibrary)
          (else
            (bind _result (Utilities|Set|ToArray (Variables|Default|GetTriggers)))
            (if (or (Variables|/Game/Elements/BP_TriggerActor.BP_TriggerActor_C|GetShouldStay? (Utilities|Array|Get(acopy) _result)) (Variables|Default|GetOneWay?))
              ;;[1 0.2 0.2] Off
              (Utilities|FlowControl|Sequence
                (:then_0
                  (bind _cube_1_to_move_4 (Variables|Refs|GetCube%201%20To%20Move)
                    (:then
                      (Rendering|SetVisibility _cube_1_to_move_4 false false)
                      (bind _cube_1_to_move_5 (Variables|Refs|GetCube%201%20To%20Move)
                        (:then
                          (Collision|SetCollisionEnabled _cube_1_to_move_5 "NoCollision"))
                        (:else)))
                    (:else)))
                (:then_1
                  (bind _front_fence_ref_3 (Variables|Refs|GetFront%20Fence%20Ref)
                    (:then
                      (Rendering|SetVisibility _front_fence_ref_3 true false)
                      (bind _front_fence_ref_4 (Variables|Refs|GetFront%20Fence%20Ref)
                        (:then
                          (Collision|SetCollisionEnabled _front_fence_ref_4 "QueryAndPhysics"))
                        (:else)))
                    (:else)))
                (:then_2
                  (bind _back_fence_ref_3 (Variables|Refs|GetBack%20Fence%20Ref)
                    (:then
                      (Rendering|SetVisibility _back_fence_ref_3 true false)
                      (bind _back_fence_ref_4 (Variables|Refs|GetBack%20Fence%20Ref)
                        (:then
                          (Collision|SetCollisionEnabled _back_fence_ref_4 "QueryAndPhysics"))
                        (:else)))
                    (:else)))
                (:then_3
                  (bind _r_fence_ref_3 (Variables|Refs|GetR%20Fence%20Ref)
                    (:then
                      (Rendering|SetVisibility _r_fence_ref_3 false false)
                      (bind _r_fence_ref_4 (Variables|Refs|GetR%20Fence%20Ref)
                        (:then
                          (Collision|SetCollisionEnabled _r_fence_ref_4 "NoCollision"))
                        (:else)))
                    (:else)))
                (:then_4
                  (bind _l_fence_ref_3 (Variables|Refs|GetL%20Fence%20Ref)
                    (:then
                      (Rendering|SetVisibility _l_fence_ref_3 false false)
                      (bind _l_fence_ref_4 (Variables|Refs|GetL%20Fence%20Ref)
                        (:then
                          (Collision|SetCollisionEnabled _l_fence_ref_4 "NoCollision"))
                        (:else)))
                    (:else))))
              (Rendering|Material|SetScalarParameterValue "/Game/Elements/Interactibles(Loris)/MP_FadeParam.MP_FadeParam" "Bridge Fade" 0.0 :!class /Script/Engine.KismetMaterialLibrary))))
        (else
          (Utilities|FlowControl|Sequence
            (:then_0
              (Transformation|SetRelativeLocation _cube_1_to_move (Math|Vector|MakeVector (.x _relativelocation) (Class|KismetMathLibrary|FInterpEaseinOut _base_y_pos (+ _base_y_pos 1e+02) _height 1.0) (.z _relativelocation)) false false))
            (:then_1
              (Transformation|SetRelativeLocation _cube_2_to_move (Math|Vector|MakeVector (.x _relativelocation_2) (* (Class|KismetMathLibrary|FInterpEaseinOut _base_y_pos (+ _base_y_pos 1e+02) _height 1.0) -1.0) (.z _relativelocation_2)) false false))))))))

(event Custom|Switch%20ON
  (bind _cube_2_to_move (Variables|Refs|GetCube%202%20To%20Move))
  (bind _base_y_pos (Variables|BasePos|GetBase%20Y%20pos))
  (bind _triggered_on_sound (Variables|SFX|GetTriggered%20On%20Sound))
  (bind _cube_1_to_move (Variables|Refs|GetCube%201%20To%20Move))
  (bind _relativelocation (Variables|/Script/Engine.SceneComponent|GetRelativeLocation _cube_1_to_move))
  (bind _relativelocation_2 (Variables|/Script/Engine.SceneComponent|GetRelativeLocation _cube_2_to_move))
  (if (Variables|Default|GetProximitySensor)
    (Utilities|IsValid _triggered_on_sound
      (:Is%20Valid
        (Audio|PlaySoundatLocation _triggered_on_sound (Transformation|GetWorldLocation (Variables|Default|GetMainMesh)) "0, 0, 0" 1.0 1.0 0.0 0 0 0 0))
      (:Is%20Not%20Valid
        _)))
  (Variables|Default|SetOn? true)
  (Utilities|FlowControl|RetriggerableDelay (Variables|Time|GetTime%20Required%20On%20Plate))
  (Variables|Time|SetRequired%20Time%20Completed%20? true)
  (if (Variables|Time|GetRequired%20Time%20Completed%20?)
    (bind _height (Timeline|Timeline Play)
      (:Update
        (if (Variables|Default|GetIsBridge?)
          (if (Variables|Default|GetOn?)
            ;[0 1 1] Bridge
            ;;[0.2 1 0.2] On
            (Utilities|FlowControl|Sequence
              (:then_0
                (bind _cube_1_to_move_2 (Variables|Refs|GetCube%201%20To%20Move)
                  (:then
                    (Rendering|SetVisibility _cube_1_to_move_2 true false)
                    (bind _cube_1_to_move_3 (Variables|Refs|GetCube%201%20To%20Move)
                      (:then
                        (Collision|SetCollisionEnabled _cube_1_to_move_3 "QueryAndPhysics"))
                      (:else)))
                  (:else)))
              (:then_1
                (bind _front_fence_ref (Variables|Refs|GetFront%20Fence%20Ref)
                  (:then
                    (Rendering|SetVisibility _front_fence_ref false false)
                    (bind _front_fence_ref_2 (Variables|Refs|GetFront%20Fence%20Ref)
                      (:then
                        (Collision|SetCollisionEnabled _front_fence_ref_2 "NoCollision"))
                      (:else)))
                  (:else)))
              (:then_2
                (bind _back_fence_ref (Variables|Refs|GetBack%20Fence%20Ref)
                  (:then
                    (Rendering|SetVisibility _back_fence_ref false false)
                    (bind _back_fence_ref_2 (Variables|Refs|GetBack%20Fence%20Ref)
                      (:then
                        (Collision|SetCollisionEnabled _back_fence_ref_2 "NoCollision"))
                      (:else)))
                  (:else)))
              (:then_3
                (bind _r_fence_ref (Variables|Refs|GetR%20Fence%20Ref)
                  (:then
                    (Rendering|SetVisibility _r_fence_ref true false)
                    (bind _r_fence_ref_2 (Variables|Refs|GetR%20Fence%20Ref)
                      (:then
                        (Collision|SetCollisionEnabled _r_fence_ref_2 "QueryAndPhysics"))
                      (:else)))
                  (:else)))
              (:then_4
                (bind _l_fence_ref (Variables|Refs|GetL%20Fence%20Ref)
                  (:then
                    (Rendering|SetVisibility _l_fence_ref true false)
                    (bind _l_fence_ref_2 (Variables|Refs|GetL%20Fence%20Ref)
                      (:then
                        (Collision|SetCollisionEnabled _l_fence_ref_2 "QueryAndPhysics"))
                      (:else)))
                  (:else))))
            (Rendering|Material|SetScalarParameterValue "/Game/Elements/Interactibles(Loris)/MP_FadeParam.MP_FadeParam" "Bridge Fade" 1.0 :!class /Script/Engine.KismetMaterialLibrary)
            (else
              (bind _result (Utilities|Set|ToArray (Variables|Default|GetTriggers)))
              (if (or (Variables|/Game/Elements/BP_TriggerActor.BP_TriggerActor_C|GetShouldStay? (Utilities|Array|Get(acopy) _result)) (Variables|Default|GetOneWay?))
                ;;[1 0.2 0.2] Off
                (Utilities|FlowControl|Sequence
                  (:then_0
                    (bind _cube_1_to_move_4 (Variables|Refs|GetCube%201%20To%20Move)
                      (:then
                        (Rendering|SetVisibility _cube_1_to_move_4 false false)
                        (bind _cube_1_to_move_5 (Variables|Refs|GetCube%201%20To%20Move)
                          (:then
                            (Collision|SetCollisionEnabled _cube_1_to_move_5 "NoCollision"))
                          (:else)))
                      (:else)))
                  (:then_1
                    (bind _front_fence_ref_3 (Variables|Refs|GetFront%20Fence%20Ref)
                      (:then
                        (Rendering|SetVisibility _front_fence_ref_3 true false)
                        (bind _front_fence_ref_4 (Variables|Refs|GetFront%20Fence%20Ref)
                          (:then
                            (Collision|SetCollisionEnabled _front_fence_ref_4 "QueryAndPhysics"))
                          (:else)))
                      (:else)))
                  (:then_2
                    (bind _back_fence_ref_3 (Variables|Refs|GetBack%20Fence%20Ref)
                      (:then
                        (Rendering|SetVisibility _back_fence_ref_3 true false)
                        (bind _back_fence_ref_4 (Variables|Refs|GetBack%20Fence%20Ref)
                          (:then
                            (Collision|SetCollisionEnabled _back_fence_ref_4 "QueryAndPhysics"))
                          (:else)))
                      (:else)))
                  (:then_3
                    (bind _r_fence_ref_3 (Variables|Refs|GetR%20Fence%20Ref)
                      (:then
                        (Rendering|SetVisibility _r_fence_ref_3 false false)
                        (bind _r_fence_ref_4 (Variables|Refs|GetR%20Fence%20Ref)
                          (:then
                            (Collision|SetCollisionEnabled _r_fence_ref_4 "NoCollision"))
                          (:else)))
                      (:else)))
                  (:then_4
                    (bind _l_fence_ref_3 (Variables|Refs|GetL%20Fence%20Ref)
                      (:then
                        (Rendering|SetVisibility _l_fence_ref_3 false false)
                        (bind _l_fence_ref_4 (Variables|Refs|GetL%20Fence%20Ref)
                          (:then
                            (Collision|SetCollisionEnabled _l_fence_ref_4 "NoCollision"))
                          (:else)))
                      (:else))))
                (Rendering|Material|SetScalarParameterValue "/Game/Elements/Interactibles(Loris)/MP_FadeParam.MP_FadeParam" "Bridge Fade" 0.0 :!class /Script/Engine.KismetMaterialLibrary))))
          (else
            (Utilities|FlowControl|Sequence
              (:then_0
                (Transformation|SetRelativeLocation _cube_1_to_move (Math|Vector|MakeVector (.x _relativelocation) (Class|KismetMathLibrary|FInterpEaseinOut _base_y_pos (+ _base_y_pos 1e+02) _height 1.0) (.z _relativelocation)) false false))
              (:then_1
                (Transformation|SetRelativeLocation _cube_2_to_move (Math|Vector|MakeVector (.x _relativelocation_2) (* (Class|KismetMathLibrary|FInterpEaseinOut _base_y_pos (+ _base_y_pos 1e+02) _height 1.0) -1.0) (.z _relativelocation_2)) false false)))))))))

(event EventBeginPlay
  (bind _cube_1_to_move (Variables|Refs|GetCube%201%20To%20Move))
  (bind _relativelocation (Variables|/Script/Engine.SceneComponent|GetRelativeLocation _cube_1_to_move))
  (Variables|BasePos|SetBase%20X%20Pos (.x _relativelocation))
  (Variables|BasePos|SetBase%20Y%20pos (.y _relativelocation))
  (Variables|BasePos|SetBase%20Z%20pos (.z _relativelocation)))

(fn ConstructionScript)

(fn Notify
  (params (Source :type BP%20Trigger%20Actor%20Object%20Reference) (Remove :type Boolean))
  (bind _triggers (Variables|Default|GetTriggers))
  (if Remove
    (Utilities|Set|RemoveItems _triggers (Utilities|Array|MakeArray Source))
    (else
      (Utilities|Set|AddItems _triggers (Utilities|Array|MakeArray Source))))
  (CallFunction|CheckActivation))

(fn CheckActivation
  (if (== (Utilities|Set|Length (Variables|Default|GetTriggers)) 0)
    (if (not (Variables|Default|GetIsActive?))
      (CallFunction|Activate))
    (elif (Variables|Default|GetIsActive?)
      (CallFunction|Deactivate))))

(fn Activate
  (bind _proxi_on_sound (Variables|SFX|GetProxi%20On%20Sound))
  (Variables|Default|SetIsActive? true)
  (Utilities|IsValid _proxi_on_sound
    (:Is%20Valid
      (Audio|PlaySoundatLocation _proxi_on_sound (Transformation|GetWorldLocation (Variables|Default|GetMainMesh)) "0, 0, 0" 1.0 1.0 0.0 0 0 0 0))
    (:Is%20Not%20Valid
      _))
  (CallFunction|SwitchON))

(fn Deactivate
  (bind _proxi_off_sound (Variables|SFX|GetProxi%20Off%20Sound))
  (Variables|Default|SetIsActive? false)
  (Utilities|IsValid _proxi_off_sound
    (:Is%20Valid
      (Audio|PlaySoundatLocation _proxi_off_sound (Transformation|GetWorldLocation (Variables|Default|GetMainMesh)) "0, 0, 0" 1.0 1.0 0.0 0 0 0 0))
    (:Is%20Not%20Valid
      _))
  (CallFunction|SwitchOFF))