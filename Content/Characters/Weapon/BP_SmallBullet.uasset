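; Small projectile Blueprint that delivers damage on overlap to enemies, the player or shields.
; BeginPlay copies Speed into the projectile movement component's initial and max speed.
; Collision overlaps use OwnerCharacter to filter pawns: enemy bullets hit only the player, other bullets only enemies, while shields are hit regardless of owner.
; Each valid target receives HitProjectileMessage with Damage and the bullet itself, which has no destroy logic here.
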(event OnComponentBeginOverlap(Collision)
  (params (OverlappedComponent :type Primitive%20Component%20Object%20Reference) (OtherActor :type Actor%20Object%20Reference) (OtherComp :type Primitive%20Component%20Object%20Reference) (OtherBodyIndex :type Integer) (bFromSweep :type Boolean) (SweepResult :type Hit%20Result%20Structure%20%28by%20ref%29))
  (bind _aspawn (Utilities|Casting|CastToPawn OtherActor)
    (:then
      (Utilities|Casting|CastToBP_EnemyBase (Variables|Default|GetOwnerCharacter)
        (:then
          (Utilities|Casting|CastToBP_EnemyBase _aspawn
            (:CastFailed
              (bind _asbp_player (Utilities|Casting|CastToBP_Player _aspawn))
              (Class|DamageInterface|HitProjectile(Message) _asbp_player (Variables|Default|GetDamage) self))))
        (:CastFailed
          (bind _asbp_enemy_base (Utilities|Casting|CastToBP_EnemyBase OtherActor))
          (Class|DamageInterface|HitProjectile(Message) _asbp_enemy_base (Variables|Default|GetDamage) self))))
    (:CastFailed
      (bind _asbp_shield (Utilities|Casting|CastToBP_Shield OtherActor))
      (Class|DamageInterface|HitProjectile(Message) _asbp_shield (Variables|Default|GetDamage) self))))

(event EventBeginPlay
  (bind _speed (Variables|Default|GetSpeed))
  (bind _projectilemovement (Variables|Default|GetProjectileMovement))
  (Variables|/Script/Engine.ProjectileMovementComponent|SetInitialSpeed _projectilemovement _speed)
  (Variables|/Script/Engine.ProjectileMovementComponent|SetMaxSpeed _projectilemovement _speed))

(event Collision|EventActorBeginOverlap
  (params (OtherActor :type Actor%20Object%20Reference)))

(event EventTick
  (params (DeltaSeconds :type Float%20%28single-precision%29)))

(fn ConstructionScript)